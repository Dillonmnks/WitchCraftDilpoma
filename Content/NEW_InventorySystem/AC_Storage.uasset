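; Storage component that holds a fixed-size array of item stacks for an inventory and mirrors it in a widget.
; Initialize builds one slot widget per Content entry, and UpdateUI pushes entries back into those widgets.
; PickUpItem targets stackable slots, then fills empty ones up to the stack limit before refreshing the UI.
; TransferItem moves only quantity between inventories, capped by free space, without copying item data or refreshing the UI.
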(event EventInitialize
  (params (UI_Widget :type Widget%20Object%20Reference))
  (bind _aswb_inventory_new (Utilities|Casting|CastToWB_InventoryNEW UI_Widget)
    (:then
      (bind _output_get (Variables|Default|SetWidget _aswb_inventory_new))
      (Widget|Panel|ClearChildren (Variables|/Game/NEW_InventorySystem/WB_InventoryNEW.WB_InventoryNEW_C|GetWrapBox _output_get))
      (Utilities|Array|Resize (Variables|Default|GetContent) (Variables|Default|GetSize))
      (for (_array_element _array_index) (Variables|Default|GetContent)
        (bind _returnvalue (UserInterface|CreateWidget "/Game/NEW_InventorySystem/WB_StorageItem.WB_StorageItem_C" 0 _array_element _array_index 0))
        (Widget|Panel|AddChild (Variables|/Game/NEW_InventorySystem/WB_InventoryNEW.WB_InventoryNEW_C|GetWrapBox (Variables|Default|GetWidget)) _returnvalue))
      (UserInterface|Viewport|AddtoViewport (Variables|Default|GetWidget) 0))
    (:CastFailed
      (Development|PrintString "Failed to set UI Widget reference."))))

(event EventUpdateUI
  (for (_array_element _array_index) (Class|PanelWidget|GetAllChildren (Variables|/Game/NEW_InventorySystem/WB_InventoryNEW.WB_InventoryNEW_C|GetWrapBox (Variables|Default|GetWidget)))
    (bind _aswb_storage_item (Utilities|Casting|CastToWB_StorageItem _array_element)
      (:then
        (Variables|/Game/NEW_InventorySystem/WB_StorageItem.WB_StorageItem_C|SetItem _aswb_storage_item (Utilities|Array|Get(acopy) (Variables|Default|GetContent) _array_index)))
      (:CastFailed
        (Development|PrintString "Failed to cast to StorageItem.")))))

(fn FindStackableSlots
  (params (ID :type String))
  (for (_array_element _array_index) (Variables|Default|GetContent)
    (if (and (Utilities|Enum|Equal(Enum) (.ID (Utilities|Struct|BreakS_Item _array_element)) ID) (< (.Quantity (Utilities|Struct|BreakS_Item _array_element)) (.MaxStackAmount (Utilities|Struct|BreakS_Item _array_element))))
      (Utilities|Array|Add (LocalVariables|Getslots) _array_index)))
  (return (LocalVariables|Getslots)))

(fn FindEmptySlots
  (for (_array_element _array_index) (Variables|Default|GetContent)
    (if (Utilities|Enum|Equal(Enum) (Utilities|Struct|BreakS_Item _array_element) "")
      (Utilities|Array|Add (LocalVariables|Getslots) _array_index)))
  (return (LocalVariables|Getslots)))

(fn TransferItem
  (params (fromInventory :type AC%20Storage%20Object%20Reference%20%28by%20ref%29) (fromIndex :type Integer) (toIndex :type Integer) (Item :type S%20Item%20Structure%20%28by%20ref%29))
  (bind _content (Variables|Default|GetContent))
  (bind _output (Utilities|Array|Get(acopy) _content toIndex))
  (bind (_id _name _thumbnail _mesh _quantity _maxstackamount) (Utilities|Struct|BreakS_Item _output))
  (if (Utilities|Enum|Equal(Enum) _id "")
    (LocalVariables|SetfreeSpace (Utilities|Struct|BreakS_Item Item))
    (else
      (LocalVariables|SetfreeSpace (- _maxstackamount _quantity))))
  (LocalVariables|SetaddedAmount (Math|Integer|Min(Integer) (LocalVariables|GetfreeSpace) (.Quantity (Utilities|Struct|BreakS_Item Item))))
  (Modify|RemoveatIndex fromInventory fromIndex (LocalVariables|GetaddedAmount))
  (Modify|AddatIndex toIndex (LocalVariables|GetaddedAmount)))

(fn RemoveatIndex
  (params (Index :type Integer%20%28by%20ref%29) (Amount :type Integer%20%28by%20ref%29))
  (bind _content (Variables|Default|GetContent))
  (bind _output (Utilities|Array|Get(acopy) _content Index))
  (bind (_id _name _thumbnail _mesh _quantity _maxstackamount) (Utilities|Struct|BreakS_Item _output))
  (bind _returnvalue (- _quantity Amount))
  (if (<= _returnvalue 0)
    (Utilities|Struct|SetmembersinS_Item _output "" "None" 0 0)
    (else
      (Utilities|Struct|SetmembersinS_Item _output _id _name _thumbnail _mesh _returnvalue _maxstackamount))))

(fn AddatIndex
  (params (Index :type Integer%20%28by%20ref%29) (Amount :type Integer%20%28by%20ref%29))
  (bind _content (Variables|Default|GetContent))
  (bind _output (Utilities|Array|Get(acopy) _content Index))
  (bind (_id _name _thumbnail _mesh _quantity _maxstackamount) (Utilities|Struct|BreakS_Item _output))
  (Utilities|Struct|SetmembersinS_Item _output _id _name _thumbnail _mesh (+ Amount _quantity) _maxstackamount))

(fn PickUpItem
  (params (Item :type BP%20Item%20Object%20Reference%20%28by%20ref%29))
  (bind _quantity (Utilities|Struct|BreakS_Item (Variables|/Game/Inventory/Blueprints/BP_Item.BP_Item_C|GetItem Item)))
  (bind (_id _name _thumbnail _mesh _quantity_2 _maxstackamount) (Utilities|Struct|BreakS_Item (Variables|/Game/Inventory/Blueprints/BP_Item.BP_Item_C|GetItem Item)))
  (bind _returnvalue (Math|Integer|Min(Integer) _quantity_2 _maxstackamount))
  (bind (_array_element _array_index) (Utilities|Array|ForEachLoopwithBreak (Searching|FindStackableSlots (Utilities|Struct|BreakS_Item (Variables|/Game/Inventory/Blueprints/BP_Item.BP_Item_C|GetItem Item))) :!label _label)
    (:LoopBody
      (if (== (Utilities|Struct|BreakS_Item (Variables|/Game/Inventory/Blueprints/BP_Item.BP_Item_C|GetItem Item)) 0)
        (goto _label Break)
        (else
          (bind _output_get (LocalVariables|SetaddAmount (Math|Integer|Min(Integer) (- (.MaxStackAmount (Utilities|Struct|BreakS_Item (Utilities|Array|Get(acopy) (Variables|Default|GetContent) _array_element))) (.Quantity (Utilities|Struct|BreakS_Item (Utilities|Array|Get(acopy) (Variables|Default|GetContent) _array_element)))) _quantity)))
          (Modify|AddatIndex _array_index _output_get)
          (Utilities|Struct|SetmembersinS_Item (Variables|/Game/Inventory/Blueprints/BP_Item.BP_Item_C|GetItem Item) (Math|Integer|Max(Integer) (- _quantity (LocalVariables|GetaddAmount)))))))
    (:Completed
      (bind _array_element_2 (Utilities|Array|ForEachLoopwithBreak (Searching|FindEmptySlots) :!label _label_2)
        (:LoopBody
          (if (== _quantity_2 0)
            (goto _label_2 Break)
            (else
              (Utilities|Struct|SetmembersinS_Item (Utilities|Array|Get(acopy) (Variables|Default|GetContent) _array_element_2) _id _name _thumbnail _mesh _returnvalue _maxstackamount)
              (Utilities|Struct|SetmembersinS_Item (Variables|/Game/Inventory/Blueprints/BP_Item.BP_Item_C|GetItem Item) (- _quantity_2 _returnvalue)))))
        (:Completed
          (CallFunction|UpdateUI))))))