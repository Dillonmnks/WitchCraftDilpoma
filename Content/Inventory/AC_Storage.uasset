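; AC_Storage is an inventory storage component that holds a StoredItems array and a UI widget for it.
; On BeginPlay it creates a WB_Explorer widget and adds it to the viewport.
; Initialize creates the configurable storage widget with a reference to the component, resizes StoredItems to Size and updates the widget.
; The event graph's call to Initialize is unconnected, so BeginPlay does not run it.
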(event EventBeginPlay
  (bind _returnvalue (UserInterface|CreateWidget "/Game/UI/WB_Explorer.WB_Explorer_C"))
  (UserInterface|Viewport|AddtoViewport _returnvalue 0))

(event EventTick
  (params (DeltaSeconds :type Float%20%28single-precision%29)))

(fn Initialize
  (bind _returnvalue (UserInterface|CreateWidget (Variables|Default|GetUI_Widget_Class) 0 self))
  (Variables|Default|SetUI_Widget _returnvalue)
  (Utilities|Array|Resize (Variables|Default|GetStoredItems) (Variables|Default|GetSize))
  (Default|Update (Variables|Default|GetUI_Widget)))