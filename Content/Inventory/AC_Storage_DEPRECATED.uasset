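; Deprecated inventory storage component that keeps items in a slot array sized on BeginPlay, treating zero quantity as empty.
; AddToInventory tops up same-named stacks via AddItemAtIndex, then spills the remainder into empty slots via AddItemAtEmptyIndex.
; AddAtIndex moves items between slots, even across inventories, by merging stacks or filling an empty target, without swapping.
; UpdateUI refreshes an inventory or hotbar widget but is not called here; AddItemToInventory is an empty stub.
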(event EventBeginPlay
  (Utilities|Array|Resize (Variables|Default|GetStoredItems) (Variables|Default|GetSize)))

(fn AddItematIndex
  (params (PlaceItem :type S%20Item%20Deprecated%20Structure%20%28by%20ref%29) (AtIndex :type Integer))
  (LocalVariables|Setindex AtIndex)
  (if (> (.maxstackamnt (Utilities|Array|Get(acopy) (Variables|Default|GetStoredItems) (LocalVariables|Getindex))) (.quantity (Utilities|Array|Get(acopy) (Variables|Default|GetStoredItems) (LocalVariables|Getindex))))
    (bind _output_get (LocalVariables|SettransferAmount (Math|Integer|Min(Integer) (- (.maxstackamnt (Utilities|Array|Get(acopy) (Variables|Default|GetStoredItems) (LocalVariables|Getindex))) (.quantity (Utilities|Array|Get(acopy) (Variables|Default|GetStoredItems) (LocalVariables|Getindex)))) (Utilities|Struct|BreakS_Item_Deprecated PlaceItem))))
    (Utilities|Struct|SetmembersinS_Item_Deprecated PlaceItem (- (Utilities|Struct|BreakS_Item_Deprecated PlaceItem) _output_get))
    (Utilities|Struct|SetmembersinS_Item_Deprecated (Utilities|Array|Get(acopy) (Variables|Default|GetStoredItems) (LocalVariables|Getindex)) (+ _output_get (.quantity (Utilities|Array|Get(acopy) (Variables|Default|GetStoredItems) (LocalVariables|Getindex)))))))

(fn AddItemtoInventory)

(fn AddItematEmptyIndex
  (params (Item :type S%20Item%20Deprecated%20Structure%20%28by%20ref%29) (Index :type Integer))
  (bind (_name _stackable _maxstackamnt _quantity _icon _mesh) (Utilities|Struct|BreakS_Item_Deprecated Item))
  (bind (_name_2 _stackable_2 _maxstackamnt_2 _quantity_2 _icon_2 _mesh_2) (Utilities|Struct|BreakS_Item_Deprecated Item))
  (bind _storeditems (Variables|Default|GetStoredItems))
  (if (Utilities|Struct|BreakS_Item_Deprecated Item)
    (Utilities|Array|SetArrayElem _storeditems Index (Utilities|Struct|MakeS_Item_Deprecated _name _stackable _maxstackamnt (Math|Integer|Min(Integer) _maxstackamnt _quantity) _icon _mesh))
    (Utilities|Struct|SetmembersinS_Item_Deprecated Item (Math|Integer|Max(Integer) (- _quantity _maxstackamnt)))
    (else
      (Utilities|Array|SetArrayElem _storeditems Index (Utilities|Struct|MakeS_Item_Deprecated _name_2 _stackable_2 _maxstackamnt_2 1 _icon_2 _mesh_2))
      (Utilities|Struct|SetmembersinS_Item_Deprecated Item (- _quantity_2 1)))))

(fn AddtoInventory
  (params (Item :type S%20Item%20Deprecated%20Structure%20%28by%20ref%29))
  (bind (_stackable _quantity) (Utilities|Struct|BreakS_Item_Deprecated Item))
  (bind (_emptyslots1 _sameitemslots1) (CallFunction|GetEmptySlots Item))
  (LocalVariables|SetemptySlots _emptyslots1)
  (bind _output_get (LocalVariables|SetsameItemSlots _sameitemslots1))
  ;[1 1 1] Stack on same item in inventory
  (bind _array_element (Utilities|Array|ForEachLoopwithBreak _output_get :!label _label)
    (:LoopBody
      (if (or (not _stackable) (<= _quantity 0))
        (goto _label Break)
        (else
          (CallFunction|AddItematIndex Item _array_element))))
    (:Completed
      ;[1 1 1] Add to empty slots
      (bind _array_element_2 (Utilities|Array|ForEachLoopwithBreak (LocalVariables|GetemptySlots) :!label _label_2)
        (:LoopBody
          (if (<= (Utilities|Struct|BreakS_Item_Deprecated Item) 0)
            (goto _label_2 Break)
            (else
              (CallFunction|AddItematEmptyIndex Item _array_element_2))))))))

(fn GetEmptySlots
  (params (item :type S%20Item%20Deprecated%20Structure))
  (for (_array_element _array_index) (Variables|Default|GetStoredItems)
    (if (== (.Quantity (Utilities|Struct|BreakS_Item_Deprecated _array_element)) 0)
      (Utilities|Array|Add (LocalVariables|GetemptySlots) _array_index)
      (elif (Utilities|Enum|Equal(Enum) (.Name (Utilities|Struct|BreakS_Item_Deprecated _array_element)) (Utilities|Struct|BreakS_Item_Deprecated item))
        (Utilities|Array|Add (LocalVariables|GetsameItemSlots) _array_index))))
  (return (LocalVariables|GetemptySlots) (LocalVariables|GetsameItemSlots)))

(fn AddatIndex
  (params (Target :type WB%20Inventory%20Item%20Object%20Reference) (Origin :type WB%20Inventory%20Item%20Object%20Reference))
  (bind _index (Variables|/Game/Inventory/WB_InventoryItem.WB_InventoryItem_C|GetIndex Origin))
  (bind _inventory (Variables|/Game/Inventory/WB_InventoryItem.WB_InventoryItem_C|GetInventory Origin))
  (bind _item (Variables|/Game/Inventory/WB_InventoryItem.WB_InventoryItem_C|GetItem Target))
  (bind _item_2 (Variables|/Game/Inventory/WB_InventoryItem.WB_InventoryItem_C|GetItem Origin))
  (bind _index_2 (Variables|/Game/Inventory/WB_InventoryItem.WB_InventoryItem_C|GetIndex Target))
  (bind _inventory_2 (Variables|/Game/Inventory/WB_InventoryItem.WB_InventoryItem_C|GetInventory Target))
  (bind (_name _stackable _maxstackamnt _quantity _icon _mesh) (Utilities|Struct|BreakS_Item_Deprecated _item))
  (bind (_name_2 _stackable_2 _maxstackamnt_2 _quantity_2 _icon_2 _mesh_2) (Utilities|Struct|BreakS_Item_Deprecated _item_2))
  (if (and _stackable (Utilities|Enum|Equal(Enum) _name _name_2))
    (LocalVariables|SetaddedAmount (Math|Integer|Min(Integer) (- _maxstackamnt _quantity) _quantity_2))
    (Utilities|Array|SetArrayElem (Variables|AC_Storage_DEPRECATED_C|GetStoredItems _inventory_2) _index_2 (Utilities|Struct|MakeS_Item_Deprecated _name _stackable _maxstackamnt (+ _quantity (LocalVariables|GetaddedAmount)) _icon _mesh))
    (Utilities|Array|SetArrayElem (Variables|AC_Storage_DEPRECATED_C|GetStoredItems _inventory) _index (Utilities|Struct|MakeS_Item_Deprecated _name_2 _stackable_2 _maxstackamnt_2 (Math|Integer|Max(Integer) (- _quantity_2 (LocalVariables|GetaddedAmount))) _icon _mesh))
    (elif (== _quantity 0)
      (LocalVariables|SetaddedAmount (Math|Integer|Min(Integer) _maxstackamnt_2 _quantity_2))
      (Utilities|Array|SetArrayElem (Variables|AC_Storage_DEPRECATED_C|GetStoredItems _inventory_2) _index_2 (Utilities|Struct|MakeS_Item_Deprecated _name_2 _stackable_2 _maxstackamnt_2 (LocalVariables|GetaddedAmount) _icon_2 _mesh_2))
      (Utilities|Array|SetArrayElem (Variables|AC_Storage_DEPRECATED_C|GetStoredItems _inventory) _index (Utilities|Struct|MakeS_Item_Deprecated _name_2 _stackable_2 _maxstackamnt_2 (- _quantity_2 (LocalVariables|GetaddedAmount)) _icon_2 _mesh_2)))))

(fn UpdateUI
  (bind _ui_widget (Variables|Default|GetUI_Widget))
  (bind _aswb_inventory (Utilities|Casting|CastToWB_Inventory _ui_widget)
    (:then
      (Default|Update _aswb_inventory))
    (:CastFailed
      (bind _aswb_hotbar (Utilities|Casting|CastToWB_Hotbar _ui_widget)
        (:then
          (Default|Update _aswb_hotbar))
        (:CastFailed
          (Development|PrintString "No matching widget found"))))))