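; BP_Item is an interactable world item that displays its item data's mesh and can be picked up by the player.
; Interface events toggle custom depth on focus and route interaction to InteractOnServer, which flips the replicated InteractToggle.
; Its OnRep passes the item to player 0's BP_MyCharacter and sets AutoDestroyWhenFinished when quantity is depleted.
; Construction applies the mesh and conditionally clears the child interaction area's custom shape.
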(event Custom|InteractOnServer
  (Variables|Default|SetInteractToggle (not (Variables|Default|GetInteractToggle))))

(event EventInterfaceInteract
  (CallFunction|InteractonServer))

(event EventInterfaceToggleFocus
  (params (Focus :type Boolean))
  (Rendering|SetRenderCustomDepth (Variables|Default|GetStaticMesh) Focus))

(fn ConstructionScript
  (bind _childactor (Variables|Default|GetChildActor))
  (bind _childactor_2 (Variables|/Script/Engine.ChildActorComponent|GetChildActor _childactor))
  (Components|StaticMesh|SetStaticMesh (Variables|Default|GetStaticMesh) (.Mesh (Utilities|Struct|BreakS_Item (Variables|Default|GetItem))))
  (if (== _childactor_2 "/Game/Player/Interaction/InteractionArea/BP_InteractionAreaCustomShape.BP_InteractionAreaCustomShape")
    (bind _asbp_interaction_area_custom_shape (Utilities|Casting|CastToBP_InteractionAreaCustomShape _childactor_2))
    (Variables|/Game/Player/Interaction/InteractionArea/BP_InteractionAreaCustomShape.BP_InteractionAreaCustomShape_C|SetCustomShape _asbp_interaction_area_custom_shape 0)))

(fn OnRepInteractToggle
  (bind _asbp_my_character (Utilities|Casting|CastToBP_MyCharacter (Game|GetPlayerCharacter 0)))
  (Default|PickUpItem _asbp_my_character (Variables|Default|GetItem))
  (if (<= (Utilities|Struct|BreakS_Item (Variables|Default|GetItem)) 0)
    (Variables|Default|SetbAutoDestroyWhenFinished true)))

(fn GetInteractionWidgetRef
  (return (Variables|Default|GetWidget)))