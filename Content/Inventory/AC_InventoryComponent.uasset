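; Inventory component that holds fixed-size inventory and hotbar item arrays and creates their widgets.
; On BeginPlay it sizes both arrays and shows the hotbar, while IA_Inventory toggles the inventory screen.
; AddItemsToInventory tops up same-name stacks, then fills empty slots, reloads the widget and returns any leftover quantity.
; DropItemOnSlot handles moves between slots, calling SwapItems for different names or TryFillSlot to merge matching ones.
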(event Custom|InitInventory
  (bind _returnvalue (UserInterface|CreateWidget "/Game/Inventory/WB_Inventory.WB_Inventory_C"))
  (Variables|Default|SetInventoryWidget _returnvalue)
  (Utilities|Array|Resize (Variables|Default|GetItems) (Variables|Default|GetSlotAmount))
  (Default|LoadInventory (Variables|Default|GetInventoryWidget) self))

(event Custom|InitHotbar
  (bind _returnvalue (UserInterface|CreateWidget "/Game/Inventory/WB_Hotbar.WB_Hotbar_C"))
  (Variables|Default|SetHotbarWidget _returnvalue)
  (Utilities|Array|Resize (Variables|Default|GetHotbarItems) (Variables|Default|GetHotbarSlotAmount))
  (Default|LoadHotbar (Variables|Default|GetHotbarWidget) self))

(event Input|EnhancedActionEvents|EnhancedInputActionIA_Inventory
  (params (ActionValue :type Boolean) (ElapsedSeconds :type Float%20%28double-precision%29) (TriggeredSeconds :type Float%20%28double-precision%29) (InputAction :type Input%20Action%20Object%20Reference :default "/Game/Player/InputActions/IA_Inventory.IA_Inventory"))
  (bind _inventorywidget (Variables|Default|GetInventoryWidget))
  (if (Widget|IsVisible (Variables|Default|GetInventoryWidget))
    (Widget|RemovefromParent _inventorywidget)
    (else
      (UserInterface|Viewport|AddtoViewport _inventorywidget 0))))

(event EventBeginPlay
  (CallFunction|InitInventory)
  (CallFunction|InitHotbar)
  (UserInterface|Viewport|AddtoPlayerScreen (Variables|Default|GetHotbarWidget)))

(event EventTick
  (params (DeltaSeconds :type Float%20%28single-precision%29)))

(fn AddItemstoInventory
  (params (Item :type S%20Item%20Structure) (ItemActor :type BP%20Item%20Object%20Reference))
  (bind _output_get (LocalVariables|SetInteractedWithItem Item))
  (LocalVariables|SetRemainingAmount (.quantity _output_get))
  (LocalVariables|SetBPItem ItemActor)
  (for (_array_element _array_index) (Variables|Default|GetItems)
    (if (== (Utilities|Struct|BreakS_Item _array_element) 0)
      (Utilities|Array|Add (LocalVariables|GetEmptySlots) _array_index)
      (elif (Utilities|Enum|Equal(Enum) (Utilities|Struct|BreakS_Item _array_element) (.Name (Utilities|Struct|BreakS_Item (LocalVariables|GetInteractedWithItem))))
        (Utilities|Array|Add (LocalVariables|GetSameItemSlots) _array_index))))
  (bind _array_element_2 (Utilities|Array|ForEachLoopwithBreak (LocalVariables|GetSameItemSlots) :!label _label)
    (:LoopBody
      (if (<= (LocalVariables|GetRemainingAmount) 0)
        (goto _label Break)
        (else
          (bind _output_get_2 (LocalVariables|SetRemainingSpace (- (.MaxStackAmnt (Utilities|Struct|BreakS_Item (Utilities|Array|Get(acopy) (Variables|Default|GetItems) _array_element_2))) (.Quantity (Utilities|Struct|BreakS_Item (Utilities|Array|Get(acopy) (Variables|Default|GetItems) _array_element_2))))))
          (LocalVariables|SetUsedAmount (Math|Integer|Min(Integer) _output_get_2 (LocalVariables|GetRemainingAmount)))
          (Utilities|Array|SetArrayElem (Variables|Default|GetItems) _array_element_2 (Utilities|Struct|MakeS_Item (.Name (Utilities|Struct|BreakS_Item (Utilities|Array|Get(acopy) (Variables|Default|GetItems) _array_element_2))) (.Stackable (Utilities|Struct|BreakS_Item (Utilities|Array|Get(acopy) (Variables|Default|GetItems) _array_element_2))) (.MaxStackAmnt (Utilities|Struct|BreakS_Item (Utilities|Array|Get(acopy) (Variables|Default|GetItems) _array_element_2))) (+ (.Quantity (Utilities|Struct|BreakS_Item (Utilities|Array|Get(acopy) (Variables|Default|GetItems) _array_element_2))) (LocalVariables|GetUsedAmount)) (.Icon (Utilities|Struct|BreakS_Item (Utilities|Array|Get(acopy) (Variables|Default|GetItems) _array_element_2))) (.Mesh (Utilities|Struct|BreakS_Item (Utilities|Array|Get(acopy) (Variables|Default|GetItems) _array_element_2)))))
          (LocalVariables|SetRemainingAmount (- (LocalVariables|GetRemainingAmount) (LocalVariables|GetUsedAmount))))))
    (:Completed
      (bind _array_element_3 (Utilities|Array|ForEachLoopwithBreak (LocalVariables|GetEmptySlots) :!label _label_2)
        (:LoopBody
          (if (<= (LocalVariables|GetRemainingAmount) 0)
            (goto _label_2 Break)
            (else
              (bind _output_get_3 (LocalVariables|SetRemainingSpace (Utilities|Struct|BreakS_Item (LocalVariables|GetInteractedWithItem))))
              (LocalVariables|SetUsedAmount (Math|Integer|Min(Integer) _output_get_3 (LocalVariables|GetRemainingAmount)))
              (Utilities|Array|SetArrayElem (Variables|Default|GetItems) _array_element_3 (Utilities|Struct|MakeS_Item (.Name (Utilities|Struct|BreakS_Item (LocalVariables|GetInteractedWithItem))) (.Stackable (Utilities|Struct|BreakS_Item (LocalVariables|GetInteractedWithItem))) (.MaxStackAmnt (Utilities|Struct|BreakS_Item (LocalVariables|GetInteractedWithItem))) (LocalVariables|GetUsedAmount) (.Icon (Utilities|Struct|BreakS_Item (LocalVariables|GetInteractedWithItem))) (.Mesh (Utilities|Struct|BreakS_Item (LocalVariables|GetInteractedWithItem)))))
              (LocalVariables|SetRemainingAmount (- (LocalVariables|GetRemainingAmount) (LocalVariables|GetUsedAmount))))))
        (:Completed
          (Default|LoadInventory (Variables|Default|GetInventoryWidget) self)
          (return (LocalVariables|GetRemainingAmount)))))))

(fn DropItemonSlot
  (params (targetIndex :type Integer) (placingIndex :type Integer) (fromSlot :type WB%20Inventory%20Item%20Object%20Reference%20%28by%20ref%29) (toSlot :type WB%20Inventory%20Item%20Object%20Reference%20%28by%20ref%29))
  (bind _index (Variables|/Game/Inventory/WB_InventoryItem.WB_InventoryItem_C|GetIndex fromSlot))
  (bind _index_2 (Variables|/Game/Inventory/WB_InventoryItem.WB_InventoryItem_C|GetIndex toSlot))
  (bind _inventory (Variables|/Game/Inventory/WB_InventoryItem.WB_InventoryItem_C|Getinventory toSlot))
  (bind _inventory_2 (Variables|/Game/Inventory/WB_InventoryItem.WB_InventoryItem_C|Getinventory fromSlot))
  (bind _output (Utilities|Array|Get(acopy) _inventory_2 _index))
  (bind _output_2 (Utilities|Array|Get(acopy) _inventory _index_2))
  (LocalVariables|SettargetInd targetIndex)
  (LocalVariables|SetplacingInd placingIndex)
  (LocalVariables|SetTargetItem _output)
  (LocalVariables|SetPlacingItem _output_2)
  (if (Utilities|Enum|NotEqual(Enum) (Utilities|Struct|BreakS_Item (LocalVariables|GetTargetItem)) (Utilities|Struct|BreakS_Item (LocalVariables|GetPlacingItem)))
    (CallFunction|SwapItems toSlot fromSlot)
    (else
      (CallFunction|TryFillSlot _output _output_2)
      (Default|LoadInventory (Variables|Default|GetInventoryWidget) self)
      (Development|PrintString (Utilities|String|ToString(Integer) (.Quantity (Utilities|Struct|BreakS_Item (LocalVariables|GetPlacingItem))))))))

(fn SwapItems
  (params (to :type WB%20Inventory%20Item%20Object%20Reference%20%28by%20ref%29) (from :type WB%20Inventory%20Item%20Object%20Reference%20%28by%20ref%29) (toInventory :type Array%20of%20S%20Item%20Structures) (toIndex :type Integer%20%28by%20ref%29) (toItem :type S%20Item%20Structure%20%28by%20ref%29))
  (bind (_name _stackable _maxstackamnt _quantity _icon _mesh) (Utilities|Struct|BreakS_Item toItem))
  (bind _inventory (Variables|/Game/Inventory/WB_InventoryItem.WB_InventoryItem_C|Getinventory to))
  (bind _index (Variables|/Game/Inventory/WB_InventoryItem.WB_InventoryItem_C|GetIndex to))
  (LocalVariables|SetplaceHolderItem (|Copy (Utilities|Array|Get(acopy) _inventory _index)))
  (Utilities|Array|SetArrayElem _inventory _index (Utilities|Struct|MakeS_Item _name _stackable _maxstackamnt _quantity _icon _mesh))
  (Utilities|Array|SetArrayElem toInventory toIndex (Utilities|Struct|MakeS_Item (.Name (Utilities|Struct|BreakS_Item (LocalVariables|GetplaceHolderItem))) (.Stackable (Utilities|Struct|BreakS_Item (LocalVariables|GetplaceHolderItem))) (.MaxStackAmnt (Utilities|Struct|BreakS_Item (LocalVariables|GetplaceHolderItem))) (.Quantity (Utilities|Struct|BreakS_Item (LocalVariables|GetplaceHolderItem))) (.Icon (Utilities|Struct|BreakS_Item (LocalVariables|GetplaceHolderItem))) (.Mesh (Utilities|Struct|BreakS_Item (LocalVariables|GetplaceHolderItem))))))

(fn TryFillSlot
  (params (targetItem :type S%20Item%20Structure%20%28by%20ref%29) (placingItem :type S%20Item%20Structure%20%28by%20ref%29) (targetInd :type Integer) (originIndex :type Integer))
  (bind (_name _stackable _maxstackamnt _quantity) (Utilities|Struct|BreakS_Item targetItem))
  (bind _quantity_2 (Utilities|Struct|BreakS_Item placingItem))
  (bind _output_get (LocalVariables|SetFreeSpace (- _maxstackamnt _quantity)))
  (bind _output_get_2 (LocalVariables|SetUsedAmount (Math|Integer|Min(Integer) _output_get _quantity_2)))
  (Utilities|Struct|SetmembersinS_Item targetItem (+ _output_get_2 _quantity))
  (Utilities|Struct|SetmembersinS_Item placingItem (- _quantity_2 (LocalVariables|GetUsedAmount))))