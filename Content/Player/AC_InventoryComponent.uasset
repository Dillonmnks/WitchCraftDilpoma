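; Player inventory component that stores items in a fixed-size slot array and shows them in a WB_Inventory widget toggled by IA_Inventory.
; AddItemsToInventory tops up stacks with the same name first, then fills empty (zero-quantity) slots up to the max stack amount.
; It reloads the widget after each slot change and returns any amount that did not fit.
; Stack matching uses name only; the Stackable check is left unconnected.
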(event Input|EnhancedActionEvents|EnhancedInputActionIA_Inventory
  (params (ActionValue :type Boolean) (ElapsedSeconds :type Float%20%28double-precision%29) (TriggeredSeconds :type Float%20%28double-precision%29) (InputAction :type Input%20Action%20Object%20Reference :default "/Game/Player/InputActions/IA_Inventory.IA_Inventory"))
  (bind _inventorywidget (Variables|Default|GetInventoryWidget))
  (if (Widget|IsVisible (Variables|Default|GetInventoryWidget))
    (Widget|RemovefromParent _inventorywidget)
    (else
      (UserInterface|Viewport|AddtoViewport _inventorywidget 0))))

(event EventBeginPlay
  (bind _returnvalue (UserInterface|CreateWidget "/Game/Inventory/WB_Inventory.WB_Inventory_C"))
  (Variables|Default|SetInventoryWidget _returnvalue)
  (Utilities|Array|Resize (Variables|Default|GetItems) 28)
  (Default|LoadInventory (Variables|Default|GetInventoryWidget) self))

(event EventTick
  (params (DeltaSeconds :type Float%20%28single-precision%29)))

(fn AddItemstoInventory
  (params (Item :type S%20Item%20Structure) (ItemActor :type BP%20Item%20Object%20Reference))
  (bind _output_get (LocalVariables|SetInteractedWithItem Item))
  (LocalVariables|SetRemainingAmount (.quantity _output_get))
  (LocalVariables|SetBPItem ItemActor)
  (for (_array_element _array_index) (Variables|Default|GetItems)
    (if (== (Utilities|Struct|BreakS_Item _array_element) 0)
      (Utilities|Array|Add (LocalVariables|GetEmptySlots) _array_index)
      (elif (Utilities|Enum|Equal(Enum) (Utilities|Struct|BreakS_Item _array_element) (.Name (Utilities|Struct|BreakS_Item (LocalVariables|GetInteractedWithItem))))
        (Utilities|Array|Add (LocalVariables|GetSameItemSlots) _array_index))))
  (bind _array_element_2 (Utilities|Array|ForEachLoopwithBreak (LocalVariables|GetSameItemSlots) :!label _label)
    (:LoopBody
      (if (<= (LocalVariables|GetRemainingAmount) 0)
        (goto _label Break)
        (else
          (bind _output_get_2 (LocalVariables|SetRemainingSpace (- (.MaxStackAmnt (Utilities|Struct|BreakS_Item (Utilities|Array|Get(acopy) (Variables|Default|GetItems) _array_element_2))) (.Quantity (Utilities|Struct|BreakS_Item (Utilities|Array|Get(acopy) (Variables|Default|GetItems) _array_element_2))))))
          (LocalVariables|SetUsedAmount (Math|Integer|Min(Integer) _output_get_2 (LocalVariables|GetRemainingAmount)))
          (Utilities|Array|SetArrayElem (Variables|Default|GetItems) _array_element_2 (Utilities|Struct|MakeS_Item (.Name (Utilities|Struct|BreakS_Item (Utilities|Array|Get(acopy) (Variables|Default|GetItems) _array_element_2))) (.Stackable (Utilities|Struct|BreakS_Item (Utilities|Array|Get(acopy) (Variables|Default|GetItems) _array_element_2))) (.MaxStackAmnt (Utilities|Struct|BreakS_Item (Utilities|Array|Get(acopy) (Variables|Default|GetItems) _array_element_2))) (+ (.Quantity (Utilities|Struct|BreakS_Item (Utilities|Array|Get(acopy) (Variables|Default|GetItems) _array_element_2))) (LocalVariables|GetUsedAmount)) (.Icon (Utilities|Struct|BreakS_Item (Utilities|Array|Get(acopy) (Variables|Default|GetItems) _array_element_2))) (.Mesh (Utilities|Struct|BreakS_Item (Utilities|Array|Get(acopy) (Variables|Default|GetItems) _array_element_2)))))
          (LocalVariables|SetRemainingAmount (- (LocalVariables|GetRemainingAmount) (LocalVariables|GetUsedAmount)))
          (Default|LoadInventory (Variables|Default|GetInventoryWidget) self))))
    (:Completed
      (bind _array_element_3 (Utilities|Array|ForEachLoopwithBreak (LocalVariables|GetEmptySlots) :!label _label_2)
        (:LoopBody
          (if (<= (LocalVariables|GetRemainingAmount) 0)
            (goto _label_2 Break)
            (else
              (bind _output_get_3 (LocalVariables|SetRemainingSpace (Utilities|Struct|BreakS_Item (LocalVariables|GetInteractedWithItem))))
              (LocalVariables|SetUsedAmount (Math|Integer|Min(Integer) _output_get_3 (LocalVariables|GetRemainingAmount)))
              (Utilities|Array|SetArrayElem (Variables|Default|GetItems) _array_element_3 (Utilities|Struct|MakeS_Item (.Name (Utilities|Struct|BreakS_Item (LocalVariables|GetInteractedWithItem))) (.Stackable (Utilities|Struct|BreakS_Item (LocalVariables|GetInteractedWithItem))) (.MaxStackAmnt (Utilities|Struct|BreakS_Item (LocalVariables|GetInteractedWithItem))) (LocalVariables|GetUsedAmount) (.Icon (Utilities|Struct|BreakS_Item (LocalVariables|GetInteractedWithItem))) (.Mesh (Utilities|Struct|BreakS_Item (LocalVariables|GetInteractedWithItem)))))
              (LocalVariables|SetRemainingAmount (- (LocalVariables|GetRemainingAmount) (LocalVariables|GetUsedAmount)))
              (Default|LoadInventory (Variables|Default|GetInventoryWidget) self))))
        (:Completed
          (return (LocalVariables|GetRemainingAmount)))))))