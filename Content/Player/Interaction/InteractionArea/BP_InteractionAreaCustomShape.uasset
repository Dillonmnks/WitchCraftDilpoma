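; Interaction area actor for the player interaction system that takes its shape from a custom static mesh.
; The construction script assigns CustomShape to the mesh component, then runs the parent construction script.
; With DEV set, every material slot gets the interaction trace shape material; otherwise the mesh is hidden without affecting its children.
; The event graph holds no active logic.
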(event EventBeginPlay)

(event Collision|EventActorBeginOverlap
  (params (OtherActor :type Actor%20Object%20Reference)))

(event EventTick
  (params (DeltaSeconds :type Float%20%28single-precision%29)))

(fn ConstructionScript
  (bind _staticmesh (Variables|Default|GetStaticMesh))
  (Components|StaticMesh|SetStaticMesh (Variables|Default|GetStaticMesh) (Variables|Default|GetCustomShape))
  (if (Variables|Default|GetDEV)
    (for _array_element (Class|PrimitiveComponent|GetMaterialSlotNames _staticmesh)
      (Rendering|Material|SetMaterialbyName (Variables|Default|GetStaticMesh) _array_element "/Game/Player/Interaction/InteractionArea/M_InteractionTraceShape.M_InteractionTraceShape"))
    (else
      (Rendering|SetVisibility _staticmesh false false)))
  (|CallParentFunction))