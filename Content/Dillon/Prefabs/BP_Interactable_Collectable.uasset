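; Interactable pickup item that places a DT_Items entry in the world and adds it to the player's inventory on interact.
; On BeginPlay it builds its item struct from the data table, sets the mesh and material, and shows name and amount in a widget.
; Collect passes the stack to BPC_PlayerInventory, keeps any leftover amount, plays a sound on any pickup, and flags auto-destroy when none remains.
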(event EventBeginPlay
  (CallFunction|InitializeItem)
  (CallFunction|UpdateUIText))

(event EventInteractNEW
  (CallFunction|Collect)
  (CallFunction|UpdateUIText))

(fn ConstructionScript
  (|CallParentFunction))

(fn Collect
  (bind _asbp_fp_hands (Utilities|Casting|CastToBP_FP_Hands (Game|GetPlayerCharacter 0))
    (:then
      (bind _returnvalue (Utilities|GetDataTableRow "/Game/Dillon/Inventory/Items/DT_Items.DT_Items" (Utilities|String|StringToName (Variables|Default|Get_Item)))
        (:then
          (bind _structout (Utilities|Struct|SetmembersinBPS_Item _returnvalue (.Amount (Utilities|Struct|BreakBPS_Item (Variables|Default|GetItem)))))
          (bind _amountleft_ (Default|AddtoInventory (Actor|GetComponentbyClass _asbp_fp_hands "/Game/Dillon/Player/BPC_PlayerInventory.BPC_PlayerInventory_C") _structout))
          (if (== _amountleft_ (.Amount (Utilities|Struct|BreakBPS_Item (Variables|Default|GetItem))))
            _
            (else
              (Class|AkGameplayStatics|PostEvent "/Game/WwiseAudio/Evemts/UI_Events/Play_Ui_item_collect.Play_Ui_item_collect")))
          (if (== _amountleft_ 0)
            (Development|PrintString "Collecte")
            (Variables|Default|SetbAutoDestroyWhenFinished true)
            (else
              (bind _structout_2 (Utilities|Struct|SetmembersinBPS_Item (Variables|Default|GetItem) _amountleft_))
              (Variables|Default|SetItem _structout_2))))
        (:RowNotFound
          (Development|PrintString "Item not foudn"))))
    (:CastFailed
      (Development|PrintString "Player Cast failed: BP_COLLECTIBLE" true true "(R=1.000000,G=0.000000,B=0.000000,A=1.000000)" 2e+01))))

(fn UpdateUIText
  (bind _item (Variables|Default|GetItem))
  (bind (_id _displayname _amount) (Utilities|Struct|BreakBPS_Item _item))
  (bind _returnvalue (Utilities|GetDataTableRow "/Game/Dillon/Inventory/Items/DT_Items.DT_Items" (Utilities|String|StringToName _id))
    (:then
      (bind _aswbp_collectible (Utilities|Casting|CastToWBP_Collectible (UserInterface|GetWidget (Variables|Default|GetWidget)))
        (:then
          (Default|UpdateDisplayText _aswbp_collectible (Utilities|String|Append (Utilities|String|ToString(Name) (.DisplayName (Utilities|Struct|BreakBPS_Item _returnvalue))) ": " (Utilities|String|ToString(Integer) _amount))))
        (:CastFailed
          (Development|PrintString "Widget Collectible failed"))))))

(fn InitializeItem
  (bind _returnvalue (Utilities|GetDataTableRow "/Game/Dillon/Inventory/Items/DT_Items.DT_Items" (Utilities|String|StringToName (Variables|Default|Get_Item)))
    (:then
      (bind _output_get (Variables|Default|SetItem (Utilities|Struct|MakeBPS_Item (.ID (Utilities|Struct|BreakBPS_Item _returnvalue)) (.DisplayName (Utilities|Struct|BreakBPS_Item _returnvalue)) (.Description (Utilities|Struct|BreakBPS_Item _returnvalue)) (Variables|Default|GetAmount) (.MaxStackAmount (Utilities|Struct|BreakBPS_Item _returnvalue)) (.Stackable (Utilities|Struct|BreakBPS_Item _returnvalue)) (.Consumable (Utilities|Struct|BreakBPS_Item _returnvalue)) (.Effect (Utilities|Struct|BreakBPS_Item _returnvalue)) (.Icon (Utilities|Struct|BreakBPS_Item _returnvalue)) (.Mesh (Utilities|Struct|BreakBPS_Item _returnvalue)) "/Game/Eleftheria_Foliage/Collectables_Whole/Flowers_Whole/flower_mat.flower_mat")))
      (Components|StaticMesh|SetStaticMesh (Variables|Default|GetStaticMesh) (.Mesh (Utilities|Struct|BreakBPS_Item _output_get)))
      (Rendering|Material|SetMaterial (Variables|Default|GetStaticMesh) 0 (.Material (Utilities|Struct|BreakBPS_Item _output_get))))))