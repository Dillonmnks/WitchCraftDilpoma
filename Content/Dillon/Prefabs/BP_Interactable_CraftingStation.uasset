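; Interactable crafting station that opens UI on the player's screen when interacted with.
; The interact event calls OnInteract, which gets the UI_Manager component from the player character and makes its master widget, inventory item widget and an image visible.
; It then immediately stops the character's movement and switches the player controller to UI-only input.
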(event Custom|Interact_1
  (CallFunction|OnInteract))

(event EventBeginPlay)

(fn ConstructionScript
  (|CallParentFunction))

(fn OnInteract
  (Widget|SetVisibility (Variables|/Game/Dillon/Player/WBP_UI_Master.WBP_UI_Master_C|GetWBP_InventoryItem (Variables|/Game/Dillon/Player/UI_Manager.UI_Manager_C|GetUI_MasterWIdget (Actor|GetComponentbyClass (Game|GetPlayerCharacter 0) "/Game/Dillon/Player/UI_Manager.UI_Manager_C"))) "Visible")
  (Components|Movement|StopMovementImmediately (Variables|/Script/Engine.Character|GetCharacterMovement (Game|GetPlayerCharacter 0)))
  (Input|SetInputModeUIOnly (Game|GetPlayerController 0) 0 "DoNotLock" false))