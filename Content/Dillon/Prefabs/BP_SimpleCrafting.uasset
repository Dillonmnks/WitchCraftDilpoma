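; Crafting station actor that turns the player's selected hotbar item into a recipe output, which is collected on a later interact for XP.
; A Data Table row keyed by item ID supplies output, cost and duration, with the player's crafting speed scaling the time.
; A finish timer runs beside a looping update timer that drains mana, pausing countdown and knife animation while mana is short.
; A widget shows remaining time or the finished item.
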(event EventBeginPlay
  (bind _asbp_fp_hands (Utilities|Casting|CastToBP_FP_Hands (Game|GetPlayerCharacter 0)))
  (Variables|Default|SetPlayer _asbp_fp_hands)
  (bind _aswbp_collectible (Utilities|Casting|CastToWBP_Collectible (UserInterface|GetWidget (Variables|Default|GetWidget))))
  (Variables|Default|SetthisWidget _aswbp_collectible))

(event EventInteractNEW
  (if (CallFunction|HasCraftedItem)
    (CallFunction|CollectCraftedItem)
    (elif (Variables|Default|GetisCrafting)
      (Class|AkGameplayStatics|PostEvent "/Game/WwiseAudio/Evemts/UI_Events/Play_Ui_item_collect_fail.Play_Ui_item_collect_fail" (Game|GetPlayerCharacter 0))
      (elif (CallFunction|IsValidInput (CallFunction|GetItemID))
        (CallFunction|StartCraftingProcess)
        (else
          (Class|AkGameplayStatics|PostEvent "/Game/WwiseAudio/Evemts/UI_Events/Play_Ui_item_collect_fail.Play_Ui_item_collect_fail" (Game|GetPlayerCharacter 0)))))))

(fn ConstructionScript
  (|CallParentFunction))

(fn HasCraftedItem
  (return (not (Utilities|Enum|Equal(Enum) (.ID (Utilities|Struct|BreakBPS_Item (Variables|Default|GetCraftedItem))) "DEFAULT_ID"))))

(fn IsValidInput
  (params (currentItemID :type String))
  (bind _returnvalue (Utilities|GetDataTableRow (Variables|Default|GetdataTable) (Utilities|String|StringToName currentItemID))
    (:then
      (Variables|Default|SetRecipe _returnvalue)
      (return true))
    (:RowNotFound
      (return false))))

(fn GetItemID
  (bind _player (Variables|Default|GetPlayer))
  (return (.ID (Utilities|Struct|BreakBPS_Item (Utilities|Array|Get(acopy) (Variables|/Game/Dillon/Player/BPC_PlayerInventory.BPC_PlayerInventory_C|GetInventory (Variables|/Game/Dillon/Player/BP_FP_Hands.BP_FP_Hands_C|GetBPC_PlayerInventory _player)) (Variables|/Game/Dillon/Player/BP_FP_Hands.BP_FP_Hands_C|GethotbarIndex _player))))))

(fn StartCraftingProcess
  (bind _recipe (Variables|Default|GetRecipe))
  (bind _player (Variables|Default|GetPlayer))
  (bind _duration (Utilities|Struct|BreakBPS_SimpleCraftingRecipe _recipe))
  (bind _craftingspeed (Default|GetCraftingSpeed _player))
  (bind _returnvalue (* _craftingspeed _duration))
  (Variables|Default|SetisCrafting true)
  (CallFunction|RemoveItemfromPlayer)
  (Variables|Default|SetManaPerUpdate (CallFunction|ManaRequired))
  (bind _returnvalue_2 (Utilities|Time|SetTimerbyFunctionName 0 "FinishCrafting" _returnvalue))
  (Variables|Default|SetTimer _returnvalue_2)
  (bind _returnvalue_3 (Utilities|Time|SetTimerbyFunctionName 0 "UpdateCrafting" (Variables|Default|GetUpdateRate) true))
  (Variables|Default|SetUpdateTimer _returnvalue_3)
  (Animation|StartAnmiation _returnvalue)
  (Development|PrintString (Utilities|String|Append "Crafting Duration: " (Utilities|String|ToString(Float) _returnvalue))))

(fn MakeCraftedItem
  (bind _returnvalue (Utilities|GetDataTableRow "/Game/Dillon/Inventory/Items/DT_Items.DT_Items" (Utilities|String|StringToName (Utilities|String|EnumtoString (.Output (Utilities|Struct|BreakBPS_SimpleCraftingRecipe (Variables|Default|GetRecipe))))))
    (:then
      (return (Utilities|Struct|MakeBPS_Item (.ID (Utilities|Struct|BreakBPS_Item _returnvalue)) (.DisplayName (Utilities|Struct|BreakBPS_Item _returnvalue)) (.Description (Utilities|Struct|BreakBPS_Item _returnvalue)) 1 (.MaxStackAmount (Utilities|Struct|BreakBPS_Item _returnvalue)) (.Stackable (Utilities|Struct|BreakBPS_Item _returnvalue)) (.Consumable (Utilities|Struct|BreakBPS_Item _returnvalue)) (.Effect (Utilities|Struct|BreakBPS_Item _returnvalue)) (.Icon (Utilities|Struct|BreakBPS_Item _returnvalue)) (.Mesh (Utilities|Struct|BreakBPS_Item _returnvalue)) (.Material (Utilities|Struct|BreakBPS_Item _returnvalue)))))))

(fn RemoveItemfromPlayer
  (bind _player (Variables|Default|GetPlayer))
  (Default|RemovefromIndex (Variables|/Game/Dillon/Player/BP_FP_Hands.BP_FP_Hands_C|GetBPC_PlayerInventory _player) (Variables|/Game/Dillon/Player/BP_FP_Hands.BP_FP_Hands_C|GethotbarIndex _player)))

(fn FinishCrafting
  (Utilities|Time|ClearandInvalidateTimerbyHandle (Variables|Default|GetUpdateTimer))
  (Utilities|Time|ClearandInvalidateTimerbyHandle (Variables|Default|GetTimer))
  (bind _item (CallFunction|MakeCraftedItem))
  (Variables|Default|SetCraftedItem _item)
  (Variables|Default|SetisCrafting false)
  (Default|UpdateDisplayText (Variables|Default|GetthisWidget) (Utilities|String|ToString(Name) (Utilities|Struct|BreakBPS_Item (Variables|Default|GetCraftedItem)))))

(fn UpdateCrafting
  (bind _timer (Variables|Default|GetTimer))
  (bind _timer_2 (Variables|Default|GetTimer))
  (bind _returnvalue (Utilities|Time|GetTimerRemainingTimebyHandle _timer))
  (bind _returnvalue_2 (Math|Timespan|FromSeconds _returnvalue))
  (bind _returnvalue_3 (Class|KismetTextLibrary|AsTimespanTimespan _returnvalue_2))
  (bind _returnvalue_4 (Utilities|String|ToString(Text) _returnvalue_3))
  (if (> (Variables|Default|GetManaPerUpdate) (Variables|/Game/Dillon/Player/BP_FP_Hands.BP_FP_Hands_C|GetMana (Variables|Default|GetPlayer)))
    (Utilities|Time|PauseTimerbyHandle (Variables|Default|GetTimer))
    (Animation|PauseAnimation)
    (Default|SetFontColor (Variables|Default|GetthisWidget) (Utilities|Struct|MakeSlateColor "(R=1.000000,G=0.000000,B=0.000000,A=1.000000)"))
    (Default|UpdateDisplayText (Variables|Default|GetthisWidget) _returnvalue_4)
    (else
      (if (Class|KismetSystemLibrary|IsTimerPausedHandle _timer_2)
        (Utilities|Time|UnpauseTimerbyHandle _timer_2)
        (Animation|UnpauseAnimation))
      (Default|SpendMana (Variables|Default|GetPlayer) (Variables|Default|GetManaPerUpdate))
      (Default|SetFontColor (Variables|Default|GetthisWidget) (Utilities|Struct|MakeSlateColor "(R=5.000000,G=5.000000,B=0.000000,A=1.000000)"))
      (Default|UpdateDisplayText (Variables|Default|GetthisWidget) _returnvalue_4))))

(fn ManaRequired
  (bind _recipe (Variables|Default|GetRecipe))
  (bind (_output _duration _cost) (Utilities|Struct|BreakBPS_SimpleCraftingRecipe _recipe))
  (return (/ _cost (/ _duration (Variables|Default|GetUpdateRate)))))

(fn StartAnmiation
  (params (InputPin :type Float%20%28double-precision%29))
  (Variables|/Script/Engine.SkeletalMeshComponent|SetGlobalAnimRateScale (Variables|Default|GetA_Knife) (/ (Animation|GetPlayLength (Variables|Default|GetAnimation)) InputPin))
  (Components|Animation|PlayAnimation (Variables|Default|GetA_Knife) (Variables|Default|GetAnimation) false))

(fn PauseAnimation
  (Variables|/Script/Engine.SkeletalMeshComponent|SetbPauseAnims (Variables|Default|GetA_Knife) true))

(fn UnpauseAnimation
  (Variables|/Script/Engine.SkeletalMeshComponent|SetbPauseAnims (Variables|Default|GetA_Knife) false))

(fn CollectCraftedItem
  (bind _thiswidget (Variables|Default|GetthisWidget))
  (Default|AddtoInventory (Variables|/Game/Dillon/Player/BP_FP_Hands.BP_FP_Hands_C|GetBPC_PlayerInventory (Variables|Default|GetPlayer)) (Variables|Default|GetCraftedItem))
  (Variables|Default|SetCraftedItem "")
  (Default|UpdateDisplayText _thiswidget "E")
  (Default|ResetColor _thiswidget)
  (Default|AddXP (Variables|Default|GetPlayer) (* (Utilities|Struct|BreakBPS_SimpleCraftingRecipe (Variables|Default|GetRecipe)) 0.1)))