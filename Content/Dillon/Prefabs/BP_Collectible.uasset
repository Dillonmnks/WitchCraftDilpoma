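; BP_Collectible is an interactable pickup that goes into the player's inventory.
; Highlight events toggle a flag and call ToggleHighlighting, which only prints TODO messages so far.
; Interacting calls PickUp, which passes the item to the player character's BPC_PlayerInventory and stores the result in Amount.
; A self-comparison of Amount then sets AutoDestroyWhenFinished, and the interaction widget getter is empty.
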(event EventOnHighlighted
  (if (not (Variables|Default|GetIsHighlighted))
    (Variables|Default|SetIsHighlighted true)
    (CallFunction|ToggleHighlighting)))

(event EventOnInteract
  (CallFunction|PickUp false))

(event EventOnHighlightedLeft
  (Variables|Default|SetIsHighlighted false)
  (CallFunction|ToggleHighlighting))

(fn ConstructionScript)

(fn GetInteractionWidgetRef
  (return 0))

(fn ToggleHighlighting
  (if (Variables|Default|GetIsHighlighted)
    (Development|PrintString "TODO: Highlight object.")
    (else
      (Development|PrintString "TODO: Un-highlight object."))))

(fn PickUp
  (params (Inventory :type Boolean%20%28by%20ref%29))
  (bind _asbp_my_character (Utilities|Casting|CastToBP_MyCharacter (Game|GetPlayerCharacter 0))
    (:then
      (bind _amountleft (Default|PickUp (Actor|GetComponentbyClass _asbp_my_character "/Game/Dillon/Player/BPC_PlayerInventory.BPC_PlayerInventory_C") self))
      (bind _output_get (Variables|Default|SetAmount _amountleft))
      (if (== (Variables|Default|GetAmount) _output_get)
        (Variables|Default|SetbAutoDestroyWhenFinished true)))
    (:CastFailed
      (Development|PrintString "Player Cast failed: BP_COLELCTIBLE" true true "(R=1.000000,G=0.000000,B=0.000000,A=1.000000)" 2e+01))))