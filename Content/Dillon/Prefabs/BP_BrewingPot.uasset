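; Brewing pot interactable that turns deposited hotbar items into potions.
; Crafting starts on left-click or at max ingredients, matching the sorted ingredient IDs against data table recipes and falling back to Gunk.
; Paired timers run the brew, draining player mana per tick and pausing countdown and duration-scaled animation when mana runs short.
; Widgets show ingredient icons on highlight, remaining time and the finished item, collected by interacting again.
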(event EventLMBInteract
  (if (not (Variables|Default|GetisCrafting))
    (CallFunction|StartCrafting)))

(event EventInteractNEW
  (if (Variables|Default|GetisCrafting)
    (CallFunction|CraftFailSound)
    (elif (CallFunction|HasCraftedItem)
      (CallFunction|CollectCraftedItem)
      (else
        (CallFunction|AddtoIngredients)
        (CallFunction|RemoveItemfromPlayer)
        (if (CallFunction|MaxIngredientsReached)
          (Development|PrintString "max ingredients" false false "(R=1.000000,G=0.005071,B=0.000000,A=1.000000)" 12.0)
          (CallFunction|StartCrafting))))))

(event EventBeginPlay
  (bind _asbp_fp_hands (Utilities|Casting|CastToBP_FP_Hands (Game|GetPlayerCharacter 0)))
  (Variables|Default|SetPlayer _asbp_fp_hands)
  (bind _aswbp_collectible (Utilities|Casting|CastToWBP_Collectible (UserInterface|GetWidget (Variables|Default|GetWidget))))
  (Variables|Default|SetthisWidget _aswbp_collectible)
  (bind _outrownames (DataTable|GetDataTableRowNames (Variables|Default|GetdataTable)))
  (Variables|Default|SetRecipes _outrownames)
  (bind _aswbp_ingredients (Utilities|Casting|CastToWBP_Ingredients (UserInterface|GetWidget (Variables|Default|GetIngredients_))))
  (Variables|Default|SetIngredientsWidget _aswbp_ingredients))

(fn ConstructionScript
  (|CallParentFunction))

(fn StartCrafting
  (if (> (Utilities|Array|Length (Variables|Default|GetIngredients)) 0)
    (bind _array_element (Utilities|Array|ForEachLoopwithBreak (Variables|Default|GetRecipes) :!label _label)
      (:LoopBody
        (bind _returnvalue (Utilities|GetDataTableRow (Variables|Default|GetdataTable) _array_element)
          (:then
            (bind _output_get (LocalVariables|SetCompareRecipe (.Ingredients (Utilities|Struct|BreakBPS_PotionRecipe _returnvalue))))
            (Class|KismetArrayLibrary|SortStringArray _output_get)
            (if (Utilities|Array|Identical (Variables|Default|GetIngredients) (LocalVariables|GetCompareRecipe))
              (Variables|Default|SetActiveRecipe _returnvalue)
              (goto _label Break)))))
      (:Completed
        (Utilities|Array|Clear (Variables|Default|GetIngredients))
        (CallFunction|UpdateIngredientsUI)
        (if (== (Utilities|Struct|BreakBPS_PotionRecipe (Variables|Default|GetActiveRecipe)) "DEFAULT_NAME")
          (bind _returnvalue_2 (Utilities|GetDataTableRow (Variables|Default|GetdataTable) "Gunk")
            (:then
              (Variables|Default|SetActiveRecipe _returnvalue_2))))
        (Variables|Default|SetisCrafting true)
        (Variables|Default|SetManaPerUpdate (CallFunction|ManaRequired))
        (bind _returnvalue_3 (Utilities|Time|SetTimerbyFunctionName 0 "FinishCrafting" (* (Default|GetCraftingSpeed (Variables|Default|GetPlayer)) (Utilities|Struct|BreakBPS_PotionRecipe (Variables|Default|GetActiveRecipe)))))
        (Variables|Default|SetTimer _returnvalue_3)
        (bind _returnvalue_4 (Utilities|Time|SetTimerbyFunctionName 0 "UpdateCrafting" (Variables|Default|GetUpdateRate) true))
        (Variables|Default|SetUpdateTimer _returnvalue_4)
        (CallFunction|StartAnmiation (* (Default|GetCraftingSpeed (Variables|Default|GetPlayer)) (Utilities|Struct|BreakBPS_PotionRecipe (Variables|Default|GetActiveRecipe))))
        (Development|PrintString (Utilities|String|Append "Crafting Duration: " (Utilities|String|ToString(Float) (* (Default|GetCraftingSpeed (Variables|Default|GetPlayer)) (Utilities|Struct|BreakBPS_PotionRecipe (Variables|Default|GetActiveRecipe))))))))))

(fn HasCraftedItem
  (return (not (Utilities|Enum|Equal(Enum) (.ID (Utilities|Struct|BreakBPS_Item (Variables|Default|GetCraftedItem))) "DEFAULT_ID"))))

(fn GetItemID
  (bind _player (Variables|Default|GetPlayer))
  (return (.ID (Utilities|Struct|BreakBPS_Item (Utilities|Array|Get(acopy) (Variables|/Game/Dillon/Player/BPC_PlayerInventory.BPC_PlayerInventory_C|GetInventory (Variables|/Game/Dillon/Player/BP_FP_Hands.BP_FP_Hands_C|GetBPC_PlayerInventory _player)) (Variables|/Game/Dillon/Player/BP_FP_Hands.BP_FP_Hands_C|GethotbarIndex _player))))))

(fn MaxIngredientsReached
  (return (>= (Utilities|Array|Length (Variables|Default|GetIngredients)) (Variables|Default|GetmaxRecipeLength))))

(fn AddtoIngredients
  (Utilities|Array|Add (Variables|Default|GetIngredients) (CallFunction|GetItemID))
  (Class|AkGameplayStatics|PostEvent "/Game/WwiseAudio/Evemts/UI_Events/Play_Ui_item_drop_mushroom.Play_Ui_item_drop_mushroom" (Game|GetPlayerCharacter 0))
  (Class|KismetArrayLibrary|SortStringArray (Variables|Default|GetIngredients))
  (CallFunction|UpdateIngredientsUI))

(fn CollectCraftedItem
  (bind _thiswidget (Variables|Default|GetthisWidget))
  (Default|AddtoInventory (Variables|/Game/Dillon/Player/BP_FP_Hands.BP_FP_Hands_C|GetBPC_PlayerInventory (Variables|Default|GetPlayer)) (Variables|Default|GetCraftedItem))
  (Variables|Default|SetCraftedItem "")
  (Default|UpdateDisplayText _thiswidget "E")
  (Default|ResetColor _thiswidget)
  (Default|AddXP (Variables|Default|GetPlayer) (* (.ManaCost (Utilities|Struct|BreakBPS_PotionRecipe (Variables|Default|GetActiveRecipe))) 0.1)))

(fn ManaRequired
  (bind _activerecipe (Variables|Default|GetActiveRecipe))
  (bind (_potionname _duration _manacost) (Utilities|Struct|BreakBPS_PotionRecipe _activerecipe))
  (return (/ _manacost (/ _duration (Variables|Default|GetUpdateRate)))))

(fn UpdateCrafting
  (bind _timer (Variables|Default|GetTimer))
  (bind _timer_2 (Variables|Default|GetTimer))
  (bind _returnvalue (Utilities|Time|GetTimerRemainingTimebyHandle _timer))
  (bind _returnvalue_2 (+ _returnvalue 1.0))
  (bind _returnvalue_3 (Math|Timespan|FromSeconds _returnvalue_2))
  (bind _returnvalue_4 (Class|KismetTextLibrary|AsTimespanTimespan _returnvalue_3))
  (bind _returnvalue_5 (Utilities|String|ToString(Text) _returnvalue_4))
  (if (> (Variables|Default|GetManaPerUpdate) (Variables|/Game/Dillon/Player/BP_FP_Hands.BP_FP_Hands_C|GetMana (Variables|Default|GetPlayer)))
    (Utilities|Time|PauseTimerbyHandle (Variables|Default|GetTimer))
    (CallFunction|PauseAnimation)
    (Default|SetFontColor (Variables|Default|GetthisWidget) (Utilities|Struct|MakeSlateColor "(R=1.000000,G=0.000000,B=0.000000,A=1.000000)"))
    (Default|UpdateDisplayText (Variables|Default|GetthisWidget) _returnvalue_5)
    (else
      (if (Class|KismetSystemLibrary|IsTimerPausedHandle _timer_2)
        (Utilities|Time|UnpauseTimerbyHandle _timer_2)
        (CallFunction|UnpauseAnimation))
      (Default|SpendMana (Variables|Default|GetPlayer) (Variables|Default|GetManaPerUpdate))
      (Default|SetFontColor (Variables|Default|GetthisWidget) (Utilities|Struct|MakeSlateColor "(R=5.000000,G=5.000000,B=0.000000,A=1.000000)"))
      (Default|UpdateDisplayText (Variables|Default|GetthisWidget) _returnvalue_5))))

(fn StartAnmiation
  (params (InputPin :type Float%20%28double-precision%29))
  (Variables|/Script/Engine.SkeletalMeshComponent|SetGlobalAnimRateScale (Variables|Default|GetSkeletalMesh) (/ (Animation|GetPlayLength (Variables|Default|GetAnimation)) InputPin))
  (Components|Animation|PlayAnimation (Variables|Default|GetSkeletalMesh) (Variables|Default|GetAnimation) false))

(fn PauseAnimation
  (Variables|/Script/Engine.SkeletalMeshComponent|SetbPauseAnims (Variables|Default|GetSkeletalMesh) true))

(fn UnpauseAnimation
  (Variables|/Script/Engine.SkeletalMeshComponent|SetbPauseAnims (Variables|Default|GetSkeletalMesh) false))

(fn FinishCrafting
  (Utilities|Time|ClearandInvalidateTimerbyHandle (Variables|Default|GetUpdateTimer))
  (Utilities|Time|ClearandInvalidateTimerbyHandle (Variables|Default|GetTimer))
  (bind _item (CallFunction|MakeCraftedItem))
  (Variables|Default|SetCraftedItem _item)
  (Variables|Default|SetisCrafting false)
  (Default|UpdateDisplayText (Variables|Default|GetthisWidget) (Utilities|String|ToString(Name) (Utilities|Struct|BreakBPS_Item (Variables|Default|GetCraftedItem))))
  (Utilities|Array|Clear (Variables|Default|GetIngredients))
  (Variables|Default|SetActiveRecipe ""))

(fn MakeCraftedItem
  (bind _returnvalue (Utilities|GetDataTableRow "/Game/Dillon/Inventory/Items/DT_Items.DT_Items" (Utilities|String|StringToName (.Output (Utilities|Struct|BreakBPS_PotionRecipe (Variables|Default|GetActiveRecipe)))))
    (:then
      (return (Utilities|Struct|MakeBPS_Item (.ID (Utilities|Struct|BreakBPS_Item _returnvalue)) (.DisplayName (Utilities|Struct|BreakBPS_Item _returnvalue)) (.Description (Utilities|Struct|BreakBPS_Item _returnvalue)) 1 (.MaxStackAmount (Utilities|Struct|BreakBPS_Item _returnvalue)) (.Stackable (Utilities|Struct|BreakBPS_Item _returnvalue)) (.Consumable (Utilities|Struct|BreakBPS_Item _returnvalue)) (.Effect (Utilities|Struct|BreakBPS_Item _returnvalue)) (.Icon (Utilities|Struct|BreakBPS_Item _returnvalue)) (.Mesh (Utilities|Struct|BreakBPS_Item _returnvalue)) (.Material (Utilities|Struct|BreakBPS_Item _returnvalue)))))))

(fn RemoveItemfromPlayer
  (bind _player (Variables|Default|GetPlayer))
  (Default|RemovefromIndex (Variables|/Game/Dillon/Player/BP_FP_Hands.BP_FP_Hands_C|GetBPC_PlayerInventory _player) (Variables|/Game/Dillon/Player/BP_FP_Hands.BP_FP_Hands_C|GethotbarIndex _player)))

(fn CraftFailSound
  (Class|AkGameplayStatics|PostEvent "/Game/WwiseAudio/Evemts/UI_Events/Play_Ui_item_collect_fail.Play_Ui_item_collect_fail" (Game|GetPlayerCharacter 0)))

(fn ToggleHighlighting
  (params (Visible :type Boolean))
  (|CallParentFunction Visible)
  (CallFunction|UpdateIngredientsUI))

(fn UpdateIngredientsUI
  (Widget|Panel|ClearChildren (Variables|/Game/Dillon/UI/WBP_Ingredients.WBP_Ingredients_C|GetWrapBox (Variables|Default|GetIngredientsWidget)))
  (if (Variables|Default|GetIsHighlighted)
    (for _array_element (Variables|Default|GetIngredients)
      (bind _returnvalue (Utilities|GetDataTableRow "/Game/Dillon/Inventory/Items/DT_Items.DT_Items" (Utilities|String|StringToName _array_element))
        (:then
          (bind _returnvalue_2 (UserInterface|CreateWidget "/Game/Dillon/UI/WBP_Ingredient_SOLO.WBP_Ingredient_SOLO_C"))
          (Appearance|SetBrushfromTexture (Variables|/Game/Dillon/UI/WBP_Ingredient_SOLO.WBP_Ingredient_SOLO_C|GetImage_69 _returnvalue_2) (.Icon (Utilities|Struct|BreakBPS_Item _returnvalue)) false)
          (Class|WrapBox|AddChildtoWrapBox (Variables|/Game/Dillon/UI/WBP_Ingredients.WBP_Ingredients_C|GetWrapBox (Variables|Default|GetIngredientsWidget)) _returnvalue_2)))))
  (Rendering|SetVisibility (Variables|Default|GetIngredients_) (Variables|Default|GetIsHighlighted) false))