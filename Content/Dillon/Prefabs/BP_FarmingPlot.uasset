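; Farming plot actor where the first-person player plants seeds and waters crops.
; Interacting looks up the held hotbar item in DT_Farmables, configures the child-actor BP_Farmable with stage meshes, durations and output item, then consumes one seed.
; LMB interaction applies the wet material and marks the plant watered.
; Update dries the soil, advances plant growth and clears the watered flag; IsPlantWatered and HasPlant are stubs.
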(event EventBeginPlay
  (bind _asbp_fp_hands (Utilities|Casting|CastToBP_FP_Hands (Game|GetPlayerCharacter 0)))
  (Variables|Default|SetPlayer _asbp_fp_hands)
  (Rendering|SetCastShadow (Variables|Default|GetStaticMesh) false))

(event EventInteractNEW
  (CallFunction|PlantSeed))

(event EventLMBInteract
  (CallFunction|Water))

(fn ConstructionScript
  (|CallParentFunction))

(fn PlantSeed
  (bind _id (Default|GetCurrentHotbarItem (Variables|Default|GetPlayer)))
  (bind _returnvalue (Utilities|GetDataTableRow "/Game/Dillon/FarmingData/DT_Farmables.DT_Farmables" (Utilities|String|StringToName _id))
    (:then
      (bind _asbp_farmable (Utilities|Casting|CastToBP_Farmable (Variables|/Script/Engine.ChildActorComponent|GetChildActor (Variables|Default|Getchild_Actor))))
      (Variables|Default|Set_plant _asbp_farmable)
      (Variables|/Game/Dillon/Prefabs/BP_Farmable.BP_Farmable_C|SetStages (Variables|Default|Get_plant) (Utilities|Array|MakeArray (.seedMesh (Utilities|Struct|BreakBPS_Farmable _returnvalue)) (.stageOneMesh (Utilities|Struct|BreakBPS_Farmable _returnvalue)) (.stageTwoMesh (Utilities|Struct|BreakBPS_Farmable _returnvalue))))
      (Variables|/Game/Dillon/Prefabs/BP_Farmable.BP_Farmable_C|SetStageDuration (Variables|Default|Get_plant) (Utilities|Array|MakeArray (.seedStageDuration (Utilities|Struct|BreakBPS_Farmable _returnvalue)) (.firstStageDuration (Utilities|Struct|BreakBPS_Farmable _returnvalue)) (.secondStageDuration (Utilities|Struct|BreakBPS_Farmable _returnvalue))))
      (Variables|/Game/Dillon/Prefabs/BP_Farmable.BP_Farmable_C|SetFinalForm (Variables|Default|Get_plant) (.outItem (Utilities|Struct|BreakBPS_Farmable _returnvalue)))
      (Default|Initialize (Variables|Default|Get_plant))
      (Default|TryRemoveItems (Variables|/Game/Dillon/Player/BP_FP_Hands.BP_FP_Hands_C|GetBPC_PlayerInventory (Variables|Default|GetPlayer)) _id 1))))

(fn IsPlantWatered)

(fn HasPlant
  (return true))

(fn Water
  (Rendering|Material|SetMaterial (Variables|Default|GetStaticMesh) 0 (Variables|Default|GetWetMat))
  (bind __plant (Variables|Default|Get_plant)
    (:then
      (Variables|/Game/Dillon/Prefabs/BP_Farmable.BP_Farmable_C|SetisWatered __plant true))
    (:else)))

(fn Update
  (Rendering|Material|SetMaterial (Variables|Default|GetStaticMesh) 0 (Variables|Default|GetDryMat))
  (bind __plant (Variables|Default|Get_plant)
    (:then
      (Default|UpdateGrowthStage __plant)
      (Variables|/Game/Dillon/Prefabs/BP_Farmable.BP_Farmable_C|SetisWatered __plant false))
    (:else)))