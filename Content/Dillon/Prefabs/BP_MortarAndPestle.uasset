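; Interactable mortar and pestle crafting station that turns the player's selected hotbar item into a new item.
; Craft looks up the held item in DT_MortarRecipes, removes one, builds the output from DT_Items and starts a timer, scaling the grinding animation to the crafting time.
; Once FinishCrafting runs, interacting again moves the output into the player's inventory.
; A widget shows the countdown, collect prompt or idle label, which reads "Cutting Board".
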(event EventBeginPlay
  (bind _aswbp_collectible (Utilities|Casting|CastToWBP_Collectible (UserInterface|GetWidget (Variables|Default|GetWidget))))
  (Variables|Default|SetthisWidget _aswbp_collectible))

(event EventTick
  (params (DeltaSeconds :type Float%20%28single-precision%29))
  (bind _outputitem (Variables|Default|GetOutputItem))
  (bind (_id _displayname) (Utilities|Struct|BreakBPS_Item _outputitem))
  (if (Variables|Default|GetisCrafting)
    (Default|UpdateDisplayText (Variables|Default|GetthisWidget) (Utilities|String|Append "Time remaining: " (Utilities|String|ToString(Text) (Class|KismetTextLibrary|AsTimespanTimespan (Math|Timespan|FromSeconds (Utilities|Time|GetTimerRemainingTimebyHandle (Variables|Default|GetTimer)))))))
    (elif (Utilities|Enum|Equal(Enum) _id "DEFAULT_ID")
      (Default|UpdateDisplayText (Variables|Default|GetthisWidget) "Cutting Board")
      (else
        (Default|UpdateDisplayText (Variables|Default|GetthisWidget) (Utilities|String|Append "Collect: " (Utilities|String|ToString(Name) _displayname)))))))

(event EventInteractNEW
  (if (not (Variables|Default|GetisCrafting))
    (if (Utilities|Enum|Equal(Enum) (.ID (Utilities|Struct|BreakBPS_Item (Variables|Default|GetOutputItem))) "DEFAULT_ID")
      (CallFunction|Craft)
      (else
        (CallFunction|CollectItem)))))

(fn ConstructionScript
  (|CallParentFunction))

(fn Craft
  (bind _a_mortar (Variables|Default|GetA_Mortar))
  (bind _asbp_fp_hands (Utilities|Casting|CastToBP_FP_Hands (Game|GetPlayerCharacter 0)))
  (if (not (Utilities|Enum|Equal(Enum) (.ID (Utilities|Struct|BreakBPS_Item (Utilities|Array|Get(acopy) (Variables|/Game/Dillon/Player/BPC_PlayerInventory.BPC_PlayerInventory_C|GetInventory (Variables|/Game/Dillon/Player/BP_FP_Hands.BP_FP_Hands_C|GetBPC_PlayerInventory _asbp_fp_hands)) (Variables|/Game/Dillon/Player/BP_FP_Hands.BP_FP_Hands_C|GethotbarIndex _asbp_fp_hands)))) "DEFAULT_ID"))
    (bind _returnvalue (Utilities|GetDataTableRow "/Game/Dillon/Crafting/DT_MortarRecipes.DT_MortarRecipes" (Utilities|String|StringToName (.ID (Utilities|Struct|BreakBPS_Item (Utilities|Array|Get(acopy) (Variables|/Game/Dillon/Player/BPC_PlayerInventory.BPC_PlayerInventory_C|GetInventory (Variables|/Game/Dillon/Player/BP_FP_Hands.BP_FP_Hands_C|GetBPC_PlayerInventory _asbp_fp_hands)) (Variables|/Game/Dillon/Player/BP_FP_Hands.BP_FP_Hands_C|GethotbarIndex _asbp_fp_hands))))))
      (:then
        (bind _success (Default|TryRemoveItems (Variables|/Game/Dillon/Player/BP_FP_Hands.BP_FP_Hands_C|GetBPC_PlayerInventory _asbp_fp_hands) (.ID (Utilities|Struct|BreakBPS_Item (Utilities|Array|Get(acopy) (Variables|/Game/Dillon/Player/BPC_PlayerInventory.BPC_PlayerInventory_C|GetInventory (Variables|/Game/Dillon/Player/BP_FP_Hands.BP_FP_Hands_C|GetBPC_PlayerInventory _asbp_fp_hands)) (Variables|/Game/Dillon/Player/BP_FP_Hands.BP_FP_Hands_C|GethotbarIndex _asbp_fp_hands)))) 1))
        (if _success
          (bind _returnvalue_2 (Utilities|GetDataTableRow "/Game/Dillon/Inventory/Items/DT_Items.DT_Items" (Utilities|String|StringToName (.Output (Utilities|Struct|BreakBPS_SimpleCraftingRecipe _returnvalue))))
            (:then
              (Variables|Default|SetOutputItem (Utilities|Struct|MakeBPS_Item (.ID (Utilities|Struct|BreakBPS_Item _returnvalue_2)) (.DisplayName (Utilities|Struct|BreakBPS_Item _returnvalue_2)) (.Description (Utilities|Struct|BreakBPS_Item _returnvalue_2)) 1 (.MaxStackAmount (Utilities|Struct|BreakBPS_Item _returnvalue_2)) (.Stackable (Utilities|Struct|BreakBPS_Item _returnvalue_2)) (.Consumable (Utilities|Struct|BreakBPS_Item _returnvalue_2)) (.Effect (Utilities|Struct|BreakBPS_Item _returnvalue_2)) (.Icon (Utilities|Struct|BreakBPS_Item _returnvalue_2)) (.Mesh (Utilities|Struct|BreakBPS_Item _returnvalue_2)) "/Game/Eleftheria_Foliage/Collectables_Whole/Flowers_Whole/flower_mat.flower_mat"))
              (bind _returnvalue_3 (Utilities|Time|SetTimerbyFunctionName 0 "FinishCrafting" (Variables|Default|GetCraftingTime)))
              (Variables|Default|SetTimer _returnvalue_3)
              (Variables|Default|SetisCrafting true)
              (Variables|/Script/Engine.SkeletalMeshComponent|SetGlobalAnimRateScale _a_mortar (/ (Animation|GetPlayLength (Variables|Default|GetAnimation)) (Variables|Default|GetCraftingTime)))
              (Components|Animation|PlayAnimation _a_mortar "/Game/Fabian_Animation/Crafting_Tools/Mortar/A_Mortar_Anim.A_Mortar_Anim" false))))))))

(fn FinishCrafting
  (Development|PrintString (Utilities|String|Append "Finished crafting: " (Utilities|String|ToString(Name) (.DisplayName (Utilities|Struct|BreakBPS_Item (Variables|Default|GetOutputItem))))))
  (Variables|Default|SetisCrafting false))

(fn CollectItem
  (bind _asbp_fp_hands (Utilities|Casting|CastToBP_FP_Hands (Game|GetPlayerCharacter 0)))
  (bind _amountleft_ (Default|AddtoInventory (Variables|/Game/Dillon/Player/BP_FP_Hands.BP_FP_Hands_C|GetBPC_PlayerInventory _asbp_fp_hands) (Variables|Default|GetOutputItem)))
  (if (== _amountleft_ 0)
    (Variables|Default|SetOutputItem "")))

(fn ToggleHighlighting
  (params (Visible :type Boolean))
  (bind _outputitem (Variables|Default|GetOutputItem))
  (bind (_id _displayname) (Utilities|Struct|BreakBPS_Item _outputitem))
  (|CallParentFunction Visible)
  (if (Variables|Default|GetisCrafting)
    (Default|UpdateDisplayText (Variables|Default|GetthisWidget) (Utilities|String|Append "Time remaining: " (Utilities|String|ToString(Text) (Class|KismetTextLibrary|AsTimespanTimespan (Math|Timespan|FromSeconds (Variables|Default|GetCraftingTime))))))
    (elif (Utilities|Enum|Equal(Enum) _id "DEFAULT_ID")
      (Default|UpdateDisplayText (Variables|Default|GetthisWidget) "Cutting Board")
      (else
        (Default|UpdateDisplayText (Variables|Default|GetthisWidget) (Utilities|String|Append "Collect: " (Utilities|String|ToString(Name) _displayname)))))))