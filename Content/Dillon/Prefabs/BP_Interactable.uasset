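; BP_Interactable is an interactable item with a static mesh and a widget that appear highlighted on focus.
; ToggleFocus flips the highlight state, and ToggleHighlighting applies it to the mesh's custom depth rendering and the widget's visibility.
; UpdateUIText looks up the item's ID in DT_Items and passes its name to the WBP_Collectible widget.
; Interact and GetInteractionWidgetRef are empty stubs.
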(event EventToggleFocus
  (bind _output_get (Variables|Default|SetIsHighlighted (not (Variables|Default|GetIsHighlighted))))
  (CallFunction|ToggleHighlighting _output_get))

(fn ConstructionScript)

(fn GetInteractionWidgetRef
  (return 0))

(fn ToggleHighlighting
  (params (Visible :type Boolean))
  (bind _output_get (Variables|Default|SetIsHighlighted Visible))
  (Rendering|SetRenderCustomDepth (Variables|Default|GetStaticMesh) _output_get)
  (Rendering|SetVisibility (Variables|Default|GetWidget) (Variables|Default|GetIsHighlighted) false))

(fn UpdateUIText
  (bind _returnvalue (Utilities|GetDataTableRow "/Game/Inventory_System/DT_Items.DT_Items" (Utilities|String|StringToName (Variables|Default|GetID)))
    (:then
      (bind _aswbp_collectible (Utilities|Casting|CastToWBP_Collectible (UserInterface|GetWidget (Variables|Default|GetWidget)))
        (:then
          (Default|UpdateDisplayText _aswbp_collectible (Utilities|Text|ToText(Name) (.Name (Utilities|Struct|BreakS_Item _returnvalue)))))
        (:CastFailed
          (Development|PrintString "Widget Collectible failed"))))))

(fn Interact
  (return ""))