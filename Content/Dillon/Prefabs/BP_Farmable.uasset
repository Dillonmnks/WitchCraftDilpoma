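; Farmable crop that grows through mesh stages on a plot and becomes a harvestable item.
; UpdateGrowthStage counts days while seeded and watered, advancing stages by their durations until the last swaps in the FinalForm mesh from DT_Items.
; Interacting when farmable adds the item to the player's inventory, keeping any leftover amount or resetting the crop once all is taken.
; Focus toggles a custom-depth highlight and widget.
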(event EventToggleFocus
  (bind _output_get (Variables|Default|SetIsHighlighted (not (Variables|Default|GetIsHighlighted))))
  (CallFunction|ToggleHighlighting _output_get))

(event EventBeginPlay
  (Components|StaticMesh|SetStaticMesh (Variables|Default|GetStaticMesh) (Utilities|Array|Get(acopy) (Variables|Default|GetStages)))
  (Rendering|Material|SetMaterial (Variables|Default|GetStaticMesh) 0 "/Game/Eleftheria_Foliage/Collectables_Whole/Flowers_Whole/flower_mat.flower_mat"))

(event EventInteractNEW
  (if (Variables|Default|GetisFarmable)
    (CallFunction|Collect)))

(fn ConstructionScript)

(fn GetInteractionWidgetRef
  (return 0))

(fn ToggleHighlighting
  (params (Visible :type Boolean))
  (bind _output_get (Variables|Default|SetIsHighlighted Visible))
  (Rendering|SetRenderCustomDepth (Variables|Default|GetStaticMesh) _output_get)
  (Rendering|SetVisibility (Variables|Default|GetWidget) (Variables|Default|GetIsHighlighted) false))

(fn UpdateUIText)

(fn UpdateGrowthStage
  (if (Variables|Default|GethasSeed)
    (if (Variables|Default|GetisWatered)
      (bind _result (Math|Integer|IncrementInt (Variables|Default|GetdaysInCurrentStage))
        (:%20%20
          (if (== _result (CallFunction|GetCurrentStageDuration))
            (if (CallFunction|IsinFinalGrowthStage)
              (CallFunction|SpawnCollectable)
              (else
                (CallFunction|EnterNextStage)))))))))

(fn IsinFinalGrowthStage
  (return (== (Variables|Default|GetcurrentStage) (- (Utilities|Array|Length (Variables|Default|GetStageDuration)) 1))))

(fn GetCurrentStageDuration
  (return (Utilities|Array|Get(acopy) (Variables|Default|GetStageDuration) (Variables|Default|GetcurrentStage))))

(fn EnterNextStage
  (Math|Integer|IncrementInt (Variables|Default|GetcurrentStage)
    (:%20%20
      (Components|StaticMesh|SetStaticMesh (Variables|Default|GetStaticMesh) (Utilities|Array|Get(acopy) (Variables|Default|GetStages) (Variables|Default|GetcurrentStage)))
      (Variables|Default|SetdaysInCurrentStage 0))))

(fn SpawnCollectable
  (bind _returnvalue (Utilities|GetDataTableRow "/Game/Dillon/Inventory/Items/DT_Items.DT_Items" (Utilities|String|StringToName (Utilities|String|EnumtoString (Variables|Default|GetFinalForm))))
    (:then
      (Components|StaticMesh|SetStaticMesh (Variables|Default|GetStaticMesh) (.Mesh (Utilities|Struct|BreakBPS_Item _returnvalue)))
      (Variables|Default|SetisFarmable true)
      (Variables|Default|SetItem (Utilities|Struct|MakeBPS_Item (.ID (Utilities|Struct|BreakBPS_Item _returnvalue)) (.DisplayName (Utilities|Struct|BreakBPS_Item _returnvalue)) (.Description (Utilities|Struct|BreakBPS_Item _returnvalue)) 1 (.MaxStackAmount (Utilities|Struct|BreakBPS_Item _returnvalue)) (.Stackable (Utilities|Struct|BreakBPS_Item _returnvalue)) (.Consumable (Utilities|Struct|BreakBPS_Item _returnvalue)) (.Effect (Utilities|Struct|BreakBPS_Item _returnvalue)) (.Icon (Utilities|Struct|BreakBPS_Item _returnvalue)) (.Mesh (Utilities|Struct|BreakBPS_Item _returnvalue)) (.Material (Utilities|Struct|BreakBPS_Item _returnvalue)))))))

(fn Collect
  (bind _asbp_fp_hands (Utilities|Casting|CastToBP_FP_Hands (Game|GetPlayerCharacter 0))
    (:then
      (bind _returnvalue (Utilities|GetDataTableRow "/Game/Dillon/Inventory/Items/DT_Items.DT_Items" (Utilities|String|StringToName (Utilities|String|EnumtoString (Variables|Default|GetFinalForm))))
        (:then
          (bind _structout (Utilities|Struct|SetmembersinBPS_Item _returnvalue (Utilities|Struct|BreakBPS_Item (Variables|Default|GetItem))))
          (bind _amountleft_ (Default|AddtoInventory (Actor|GetComponentbyClass _asbp_fp_hands "/Game/Dillon/Player/BPC_PlayerInventory.BPC_PlayerInventory_C") _structout))
          (if (== _amountleft_ (Utilities|Struct|BreakBPS_Item (Variables|Default|GetItem)))
            _
            (else
              (Class|AkGameplayStatics|PostEvent "/Game/WwiseAudio/Evemts/UI_Events/Play_Ui_item_collect.Play_Ui_item_collect")))
          (if (== _amountleft_ 0)
            (Development|PrintString "Collecte")
            (Components|StaticMesh|SetStaticMesh (Variables|Default|GetStaticMesh) 0)
            (Variables|Default|SetisFarmable false)
            (Variables|Default|SetcurrentStage 0)
            (Variables|Default|SetItem "")
            (Variables|Default|SetdaysInCurrentStage 0)
            (Variables|Default|SethasSeed false)
            (else
              (bind _structout_2 (Utilities|Struct|SetmembersinBPS_Item (Variables|Default|GetItem) _amountleft_))
              (Variables|Default|SetItem _structout_2))))
        (:RowNotFound
          (Development|PrintString "Item not foudn"))))
    (:CastFailed
      (Development|PrintString "Player Cast failed: BP_COLLECTIBLE" true true "(R=1.000000,G=0.000000,B=0.000000,A=1.000000)" 2e+01))))

(fn Initialize
  (params (plot :type BP%20Farming%20Plot%20Object%20Reference))
  (Variables|Default|Setplot plot)
  (bind _returnvalue (Utilities|GetDataTableRow "/Game/Dillon/Inventory/Items/DT_Items.DT_Items" (Utilities|String|StringToName (Utilities|String|EnumtoString (Variables|Default|GetFinalForm))))
    (:then
      (Variables|Default|SetItem _returnvalue)
      (Components|StaticMesh|SetStaticMesh (Variables|Default|GetStaticMesh) (Utilities|Array|Get(acopy) (Variables|Default|GetStages))))))

(fn InteractDeprecated
  (return ""))