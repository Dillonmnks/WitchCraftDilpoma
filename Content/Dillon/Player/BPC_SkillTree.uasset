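; Player skill tree component that applies percentage increases to four stats: move speed, XP gain, crafting speed and pick up rate.
; EditModifier switches on the chosen stat, grows its stored modifier through ModifyValue, then recomputes the stat as base plus modifier.
; ModifyValue takes each percentage from the base value, so repeated increases stack additively rather than compounding.
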(fn EditModifier
  (params (Modifier :type E_PlayerStats%20Enum :default "NewEnumerator2") (increaseAmountInPercent :type Float%20%28double-precision%29))
  (switch Utilities|FlowControl|Switch|SwitchonE_PlayerStats Modifier
    (:NewEnumerator2
      (Development|PrintString "No Modifier selected to change."))
    (:NewEnumerator0
      (bind _output_get (Variables|PlayerModifiers|SetSpeedModifier (Private|ModifyValue (Variables|PlayerModifiers|GetSpeedModifier) (Variables|BaseStats|GetBaseSpeed) increaseAmountInPercent)))
      (Variables|Stats|SetMoveSpeed (+ _output_get (Variables|BaseStats|GetBaseSpeed))))
    (:NewEnumerator3
      (bind _output_get_2 (Variables|PlayerModifiers|SetXPModifier (Private|ModifyValue (Variables|PlayerModifiers|GetXPModifier) (Variables|BaseStats|GetBaseXPGain) increaseAmountInPercent)))
      (Variables|Stats|SetXPGain (+ _output_get_2 (Variables|BaseStats|GetBaseXPGain))))
    (:NewEnumerator1
      (bind _output_get_3 (Variables|PlayerModifiers|SetCraftingSpeedModifier (Private|ModifyValue (Variables|PlayerModifiers|GetCraftingSpeedModifier) (Variables|BaseStats|GetBaseCraftingSpeed) increaseAmountInPercent)))
      (Variables|Stats|SetCraftingSpeed (+ _output_get_3 (Variables|BaseStats|GetBaseCraftingSpeed))))
    (:NewEnumerator4
      (bind _output_get_4 (Variables|PlayerModifiers|SetPickUpRateModifier (Private|ModifyValue (Variables|PlayerModifiers|GetPickUpRateModifier) (Variables|BaseStats|GetBasePickUpRate) increaseAmountInPercent)))
      (Variables|Stats|SetPickUpRate (+ _output_get_4 (Variables|BaseStats|GetBasePickUpRate))))))

(fn ModifyValue
  (params (Modifier :type Float%20%28double-precision%29) (BaseValue :type Float%20%28double-precision%29) (Percent :type Float%20%28double-precision%29))
  (return (+ Modifier (* BaseValue (* Percent 0.01)))))