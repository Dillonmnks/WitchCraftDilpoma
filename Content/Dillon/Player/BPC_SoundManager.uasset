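; BPC_SoundManager is a player sound manager Blueprint that applies audio volume settings to the game's mix.
; Its UpdateSounds function takes new master, music, effects and dialogue levels and stores each in its own volume variable.
; It then pushes the stored values to matching Wwise RTPCs, leaving the audio engine to control how each level affects the sound.
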(fn UpdateSounds
  (params (newMaster :type Float%20%28double-precision%29) (newMusic :type Float%20%28double-precision%29) (newFX :type Float%20%28double-precision%29) (newDialogue :type Float%20%28double-precision%29))
  (Variables|Default|SetMasterVolume newMaster)
  (Variables|Default|SetMusicVolume newMusic)
  (Variables|Default|SetFXVolume newFX)
  (Variables|Default|SetDialogueVolume newDialogue)
  (Class|AkGameplayStatics|SetRTPCValue "/Game/WwiseAudio/Busse/Master_Volume.Master_Volume" (Variables|Default|GetMasterVolume))
  (Class|AkGameplayStatics|SetRTPCValue "/Game/WwiseAudio/Busse/Dialogue.Dialogue" (Variables|Default|GetDialogueVolume))
  (Class|AkGameplayStatics|SetRTPCValue "/Game/WwiseAudio/Busse/Music.Music" (Variables|Default|GetMusicVolume))
  (Class|AkGameplayStatics|SetRTPCValue "/Game/WwiseAudio/Busse/SFX.SFX" (Variables|Default|GetFXVolume)))