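; Player inventory component that stores items as BPS_Item structs in a fixed-size slot array, with DEFAULT_ID marking empty slots.
; Adding items, inventory-wide or within an index range, walks slots in order, filling empty slots or matching stacks and returning the leftover.
; Also handles count-checked removal by ID, single-unit removal by index, drag-drop merge or swap, and Wwise drop/consume sounds.
; Slot writes when adding items hard-code the material to Flower_mat.
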(event EventBeginPlay
  (Private|Initialize))

(fn AddtoInventory
  (params (Collectible :type BPS%20Item%20Structure))
  (LocalVariables|SetItem Collectible)
  (bind (_array_element _array_index) (Utilities|Array|ForEachLoopwithBreak (Variables|Default|GetInventory) :!label _label)
    (:LoopBody
      (LocalVariables|Setindex _array_index)
      (bind _isempty (Private|IsEmpty _array_element))
      (if _isempty
        (bind _amountleft (Private|AddatEmptyIndex (LocalVariables|GetItem) (LocalVariables|Getindex)))
        (Utilities|Struct|SetmembersinBPS_Item (LocalVariables|GetItem) _amountleft)
        (if (<= (.Amount (Utilities|Struct|BreakBPS_Item (LocalVariables|GetItem))) 0) :!label _label_2
          (goto _label Break))
        (else
          (bind _valid (Private|IsValidPosition (LocalVariables|GetItem) _array_element))
          (if _valid
            (bind _amountleft_2 (Private|AddtoExistingItem (LocalVariables|Getindex) (LocalVariables|GetItem)))
            (Utilities|Struct|SetmembersinBPS_Item (LocalVariables|GetItem) _amountleft_2)
            (goto _label_2)))))
    (:Completed
      (return (.Amount (Utilities|Struct|BreakBPS_Item (LocalVariables|GetItem)))))))

(fn Initialize
  (Utilities|Array|Resize (Variables|Default|GetInventory) (Variables|Default|GetInventorySize)))

(fn Contains
  (params (ItemID :type String) (Amount :type Integer))
  (bind _array_element (Utilities|Array|ForEachLoopwithBreak (Variables|Default|GetInventory) :!label _label)
    (:LoopBody
      (if (Utilities|Enum|Equal(Enum) (.ID (Utilities|Struct|BreakBPS_Item _array_element)) ItemID)
        (bind _output_get (LocalVariables|SetFoundAmount (+ (LocalVariables|GetFoundAmount) (.Amount (Utilities|Struct|BreakBPS_Item _array_element)))))
        (if (>= _output_get Amount)
          (goto _label Break))))
    (:Completed
      (return (>= (LocalVariables|GetFoundAmount) Amount)))))

(fn IsValidPosition
  (params (inItem :type BPS%20Item%20Structure) (inventoryItem :type BPS%20Item%20Structure))
  (bind (_id _displayname _amount _maxstackamount _stackable) (Utilities|Struct|BreakBPS_Item inventoryItem))
  (return (Math|Boolean|ANDBoolean (Utilities|Enum|Equal(Enum) (.ID (Utilities|Struct|BreakBPS_Item inItem)) _id) (< _amount _maxstackamount) _stackable)))

(fn IsEmpty
  (params (item :type BPS%20Item%20Structure))
  (return (Utilities|Enum|Equal(Enum) (.ID (Utilities|Struct|BreakBPS_Item item)) "DEFAULT_ID")))

(fn AddatEmptyIndex
  (params (item :type BPS%20Item%20Structure) (index :type Integer))
  (bind (_id _displayname _description _amount _maxstackamount _stackable _consumable _effect _icon _mesh) (Utilities|Struct|BreakBPS_Item item))
  (LocalVariables|SetAmountAdded (Math|Integer|Min(Integer) _amount _maxstackamount))
  (Development|PrintString (Utilities|String|Append "Stackable: " (Utilities|String|ToString(Boolean) _stackable)))
  (Utilities|Array|SetArrayElem (Variables|Default|GetInventory) index (Utilities|Struct|MakeBPS_Item _id _displayname _description (LocalVariables|GetAmountAdded) _maxstackamount _stackable _consumable _effect _icon _mesh "/Game/Eleftheria_Foliage/Collectables_Whole/Flowers_Whole/flower_mat.flower_mat"))
  (return (Math|Integer|Max(Integer) (- (.Amount (Utilities|Struct|BreakBPS_Item item)) (LocalVariables|GetAmountAdded)))))

(fn AddtoExistingItem
  (params (Index :type Integer) (item :type BPS%20Item%20Structure))
  (bind _inventory (Variables|Default|GetInventory))
  (bind _output (Utilities|Array|Get(acopy) _inventory Index))
  (bind (_id _displayname _description _amount _maxstackamount _stackable _consumable _effect _icon _mesh) (Utilities|Struct|BreakBPS_Item _output))
  (bind _output_get (LocalVariables|SetavailableSpace (Math|Integer|Max(Integer) (- _maxstackamount _amount))))
  (LocalVariables|SetAddAmount (Math|Integer|Min(Integer) _output_get (.Amount (Utilities|Struct|BreakBPS_Item item))))
  (Utilities|Array|SetArrayElem (Variables|Default|GetInventory) Index (Utilities|Struct|MakeBPS_Item _id _displayname _description (+ _amount (LocalVariables|GetAddAmount)) _maxstackamount _stackable _consumable _effect _icon _mesh "/Game/Eleftheria_Foliage/Collectables_Whole/Flowers_Whole/flower_mat.flower_mat"))
  (return (- (.Amount (Utilities|Struct|BreakBPS_Item item)) (LocalVariables|GetAddAmount))))

(fn TryRemoveItems
  (params (itemID :type String) (RemoveAmount :type Integer))
  (bind _inventory (Variables|Default|GetInventory))
  (bind _output_get (LocalVariables|Set_removeAmount RemoveAmount))
  (bind _out (Public|Contains itemID _output_get))
  (if _out
    (bind (_array_element _array_index) (Utilities|Array|ForEachLoopwithBreak (Variables|Default|GetInventory) :!label _label)
      (:LoopBody
        (LocalVariables|SetCurrentIndex _array_index)
        (if (Utilities|Enum|Equal(Enum) (.ID (Utilities|Struct|BreakBPS_Item _array_element)) itemID)
          (if (> (.Amount (Utilities|Struct|BreakBPS_Item _array_element)) (LocalVariables|Get_removeAmount))
            (bind _structout (Utilities|Struct|SetmembersinBPS_Item _array_element (- (.Amount (Utilities|Struct|BreakBPS_Item _array_element)) (LocalVariables|Get_removeAmount))))
            (Utilities|Array|SetArrayElem _inventory (LocalVariables|GetCurrentIndex) _structout)
            (goto _label Break)
            (else
              (LocalVariables|Set_removeAmount (- (LocalVariables|Get_removeAmount) (.Amount (Utilities|Struct|BreakBPS_Item _array_element))))
              (Utilities|Array|SetArrayElem _inventory (LocalVariables|GetCurrentIndex) (Utilities|Struct|MakeBPS_Item "DEFAULT_ID" "None" "" 1 999 false false "(Modifier_12_85AC02A2448D093D0A649282713A8640=NewEnumerator2,Amount_11_58458151459E911108A4C5B03FE3E28B=0.000000,baseModifier_8_A08F01E84A67658D5B33E0B0AA6F2980=True)" "/Game/UI/Textures_UI/Elef_Icons/Placholder_Potion_Icon/Icon_PLACEHOLDER_Potion.Icon_PLACEHOLDER_Potion" "/Game/FPWeapon/Mesh/FirstPersonProjectileMesh.FirstPersonProjectileMesh" "/Game/Eleftheria_Foliage/Collectables_Whole/Flowers_Whole/flower_mat.flower_mat"))
              (if (== (LocalVariables|Get_removeAmount) 0)
                (goto _label Break))))))
      (:Completed
        (return true)))
    (else
      (return false))))

(fn RemovefromIndex
  (params (index :type Integer))
  (bind _inventory (Variables|Default|GetInventory))
  (bind _output (Utilities|Array|Get(acopy) _inventory index))
  (bind _amount (Utilities|Struct|BreakBPS_Item _output))
  (bind _returnvalue (- _amount 1))
  (if (< _returnvalue 1)
    (Utilities|Array|SetArrayElem :TargetArray _inventory :Index index)
    (else
      (Utilities|Struct|SetmembersinBPS_Item _output _returnvalue))))

(fn OnDragDrop
  (params (fromIndex :type Integer) (toIndex :type Integer))
  (bind _inventory (Variables|Default|GetInventory))
  (bind _inventory_2 (Variables|Default|GetInventory))
  (bind _output (Utilities|Array|Get(acopy) _inventory_2 toIndex))
  (bind _output_2 (Utilities|Array|Get(acopy) _inventory_2 fromIndex))
  (bind (_id _displayname _description _amount) (Utilities|Struct|BreakBPS_Item _output_2))
  (bind (_id_2 _displayname_2 _description_2 _amount_2 _maxstackamount) (Utilities|Struct|BreakBPS_Item _output))
  (bind _returnvalue (- _maxstackamount _amount_2))
  (if (!= fromIndex toIndex)
    (if (Utilities|Enum|Equal(Enum) _id _id_2)
      (if (> _returnvalue 0)
        (bind _output_get (LocalVariables|SettransferAmount (Math|Integer|Min(Integer) _amount _returnvalue)))
        (if (== (- _amount _output_get) 0)
          (Utilities|Array|SetArrayElem :TargetArray (Variables|Default|GetInventory) :Index fromIndex)
          (else
            (Utilities|Struct|SetmembersinBPS_Item (Utilities|Array|Get(acopy) _inventory fromIndex) (- _amount _output_get))))
        (Utilities|Struct|SetmembersinBPS_Item (Utilities|Array|Get(acopy) _inventory toIndex) (+ _output_get _amount_2)))
      (else
        (Utilities|Array|Swap (Variables|Default|GetInventory) fromIndex toIndex)))))

(fn TransfertoRange
  (params (minIndex :type Integer) (maxIndex :type Integer) (item :type BPS%20Item%20Structure))
  (LocalVariables|Set_item item)
  (bind _index (Utilities|FlowControl|ForLoopwithBreak minIndex maxIndex :!label _label)
    (:LoopBody
      (bind _output_get (LocalVariables|Setindex _index))
      (bind _isempty (Private|IsEmpty (Utilities|Array|Get(acopy) (Variables|Default|GetInventory) _output_get)))
      (if _isempty
        (bind _amountleft (Private|AddatEmptyIndex (LocalVariables|Get_item) (LocalVariables|Getindex)))
        (Utilities|Struct|SetmembersinBPS_Item (LocalVariables|Get_item) _amountleft)
        (if (<= (.Amount (Utilities|Struct|BreakBPS_Item (LocalVariables|Get_item))) 0) :!label _label_2
          (goto _label Break))
        (else
          (bind _valid (Private|IsValidPosition (LocalVariables|Get_item) (Utilities|Array|Get(acopy) (Variables|Default|GetInventory) _output_get)))
          (if _valid
            (bind _amountleft_2 (Private|AddtoExistingItem (LocalVariables|Getindex) (LocalVariables|Get_item)))
            (Utilities|Struct|SetmembersinBPS_Item (LocalVariables|Get_item) _amountleft_2)
            (goto _label_2)))))
    (:Completed
      (return (.Amount (Utilities|Struct|BreakBPS_Item (LocalVariables|Get_item)))))))

(fn DropItemSound
  (Class|AkGameplayStatics|PostEvent "/Game/WwiseAudio/Evemts/UI_Events/Play_Ui_item_drop_mushroom.Play_Ui_item_drop_mushroom" (Game|GetPlayerCharacter 0)))

(fn ConsumePotion
  (Class|AkGameplayStatics|PostEvent "/Game/WwiseAudio/Evemts/UI_Events/Play_Ui_item_use_potion.Play_Ui_item_use_potion" (Game|GetPlayerCharacter 0)))

(fn ConsumeFood
  (Class|AkGameplayStatics|PostEvent "/Game/WwiseAudio/Evemts/UI_Events/Play_Ui_item_use_eat.Play_Ui_item_use_eat" (Game|GetPlayerCharacter 0)))