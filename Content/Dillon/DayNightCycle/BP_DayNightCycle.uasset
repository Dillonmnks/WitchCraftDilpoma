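; Day/night cycle actor that runs a repeating, timed in-game day and switches Wwise day and night music on the player character.
; StartDay sets timers for EndDay and for night music at 58% of the day; EndDay notifies BP_FP_Hands, then restarts.
; SwitchMaterials sets the SKY-tagged mesh's skybox material by stage, but runs only at BeginPlay.
; Stage-progression helpers exist but are never called, so the stage stays Morning.
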(event EventBeginPlay
  (bind _outactors (Actor|GetAllActorswithTag "SKY"))
  (bind _asstatic_mesh_actor (Utilities|Casting|CastToStaticMeshActor (Utilities|Array|Get(acopy) _outactors)))
  (bind _output_get (Variables|Default|SetSkyLight _asstatic_mesh_actor))
  (Development|PrintString (Utilities|GetObjectName _output_get))
  (CallFunction|StartDay)
  (bind _output_get_2 (Variables|Default|SetMiddayToEvening (+ (Variables|Default|GetMorningToMidday) (Variables|Default|GetMiddayToEvening))))
  (Variables|Default|SetEveningToNight (+ _output_get_2 (Variables|Default|GetEveningToNight)))
  (CallFunction|SwitchMaterials))

(fn ConstructionScript)

(fn StartDay
  (bind _daydurationinminutes (Variables|Default|GetDayDurationInMinutes))
  (bind _returnvalue (* _daydurationinminutes 6e+01))
  (bind _returnvalue_2 (Utilities|Time|SetTimerbyFunctionName 0 "EndDay" (* (Variables|Default|GetDayDurationInMinutes) 6e+01)))
  (Variables|Default|SetTimer _returnvalue_2)
  (Variables|Default|SetCurrentStage "NewEnumerator0")
  (Development|PrintString "timer started")
  (Class|AkGameplayStatics|SetSwitch "/Game/WwiseAudio/Switches/DayNightCycle/DayNightCycle-Day.DayNightCycle-Day" (Game|GetPlayerCharacter 0))
  (Development|PrintString "day music playing" true true "(R=0.000000,G=0.660000,B=1.000000,A=1.000000)" 2e+01)
  (Utilities|Time|SetTimerbyFunctionName 0 "ToggleMusic" (- _returnvalue (* _returnvalue 0.42))))

(fn SwitchSkyLight)

(fn EndDay
  (Utilities|Time|ClearandInvalidateTimerbyHandle (Variables|Default|GetTimer))
  (bind _asbp_fp_hands (Utilities|Casting|CastToBP_FP_Hands (Game|GetPlayerCharacter 0)))
  (Default|EndDay _asbp_fp_hands)
  (CallFunction|StartDay))

(fn CurrentStageDuration
  (switch Utilities|FlowControl|Switch|SwitchonBPE_DayTimes (Variables|Default|GetCurrentStage)
    (:NewEnumerator0
      (return (CallFunction|GetTimeinSeconds (Variables|Default|GetMorningToMidday))))
    (:NewEnumerator1
      (return (CallFunction|GetTimeinSeconds (Variables|Default|GetMiddayToEvening))))
    (:NewEnumerator2
      (return (CallFunction|GetTimeinSeconds (Variables|Default|GetEveningToNight))))
    (:NewEnumerator3
      (return (CallFunction|GetTimeinSeconds (Variables|Default|GetDayDurationInMinutes))))))

(fn GetNextStage
  (switch Utilities|FlowControl|Switch|SwitchonBPE_DayTimes (Variables|Default|GetCurrentStage)
    (:NewEnumerator0
      (return "NewEnumerator1"))
    (:NewEnumerator1
      (return "NewEnumerator2"))
    (:NewEnumerator2
      (return "NewEnumerator3"))
    (:NewEnumerator3
      (return "NewEnumerator0"))))

(fn GetTimeinSeconds
  (params (Minutes :type Float%20%28single-precision%29))
  (return (Math|Conversions|ToFloat(Integer) (.Seconds (Math|Timespan|BreakTimespan (Class|KismetMathLibrary|FromMinutes Minutes))))))

(fn SwitchMaterials
  (bind _skylight (Variables|Default|GetSkyLight))
  (bind _staticmeshcomponent (Variables|/Script/Engine.StaticMeshActor|GetStaticMeshComponent _skylight))
  (switch Utilities|FlowControl|Switch|SwitchonBPE_DayTimes (Variables|Default|GetCurrentStage)
    (:NewEnumerator0
      (Rendering|Material|SetMaterial _staticmeshcomponent 0 "/Game/SkyStuff/M_SkyboxEveningMorning.M_SkyboxEveningMorning"))
    (:NewEnumerator1
      (Rendering|Material|SetMaterial _staticmeshcomponent 0 "/Game/SkyStuff/M_SkyboxMidday.M_SkyboxMidday"))
    (:NewEnumerator2
      (Rendering|Material|SetMaterial _staticmeshcomponent 0 "/Game/SkyStuff/M_SkyboxEveningMorning.M_SkyboxEveningMorning"))
    (:NewEnumerator3
      (Rendering|Material|SetMaterial _staticmeshcomponent 0 "/Game/SkyStuff/M_SkyboxNight.M_SkyboxNight"))))

(fn ToggleMusic
  (Class|AkGameplayStatics|SetSwitch "/Game/WwiseAudio/Switches/DayNightCycle/DayNightCycle-Night.DayNightCycle-Night" (Game|GetPlayerCharacter 0))
  (Development|PrintString "night music playing" true true "(R=1.000000,G=0.345784,B=0.000000,A=1.000000)" 2e+01))