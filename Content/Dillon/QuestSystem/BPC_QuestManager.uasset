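; Quest manager component that holds active and inactive quest lists, spawns new quests and pays out rewards on completion.
; BeginPlay caches row names from QuestsDataTable; SpawnNewQuests rolls a chance while under the inactive cap, re-picks randomly past duplicates, then reads DT_Quests directly.
; CompleteQuest matches an active quest by required item, calls inventory removal with the quest's ID, grants rewards through BP_FP_Hands and drops the quest.
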(event EventBeginPlay
  (bind _questsdatatable (Variables|Default|GetQuestsDataTable)
    (:then
      (bind _outrownames (DataTable|GetDataTableRowNames _questsdatatable))
      (Variables|Default|SetAllQuests _outrownames))
    (:else)))

(fn SpawnNewQuests
  (if (< (Utilities|Array|Length (Variables|Default|GetInactiveQuests)) (Variables|Default|GetMaxInactiveQuests))
    (if (<= (Math|Random|RandomIntegerinRange 0 99) (Variables|Default|GetQuestSpawnChance))
      (bind (_ispresent _questid) (CallFunction|QuestAlreadyGiven (.OutItem (Utilities|Array|Random (Variables|Default|GetAllQuests))) :!label _label))
      (if _ispresent
        (goto _label)
        (else
          (bind _returnvalue (Utilities|GetDataTableRow "/Game/Dillon/QuestSystem/DT_Quests.DT_Quests" _questid)
            (:then
              (Utilities|Array|Add (Variables|Default|GetInactiveQuests) _returnvalue))))))))

(fn QuestAlreadyGiven
  (params (quest :type Name))
  (for _array_element (Variables|Default|GetActiveQuests)
    (if (Utilities|Enum|Equal(Enum) (.ID (Utilities|Struct|BreakBPS_Quest _array_element)) (Utilities|String|ToString(Name) quest))
      (return true quest)))
  (for _array_element_2 (Variables|Default|GetInactiveQuests)
    (if (Utilities|Enum|Equal(Enum) (.ID (Utilities|Struct|BreakBPS_Quest _array_element_2)) (Utilities|String|ToString(Name) quest))
      (return true quest)))
  (return false quest))

(fn CompleteQuest
  (params (ItemID :type String))
  (bind (_array_element _array_index) (Utilities|Array|ForEachLoopwithBreak (Variables|Default|GetActiveQuests) :!label _label)
    (:LoopBody
      (if (Utilities|Enum|Equal(Enum) (Utilities|Struct|BreakBPS_Quest _array_element) ItemID)
        (LocalVariables|Setindex _array_index)
        (bind _asbp_fp_hands (Utilities|Casting|CastToBP_FP_Hands (Game|GetPlayerCharacter 0)))
        (Default|TryRemoveItems (Variables|/Game/Dillon/Player/BP_FP_Hands.BP_FP_Hands_C|GetBPC_PlayerInventory _asbp_fp_hands) (.ID (Utilities|Struct|BreakBPS_Quest _array_element)) (.RequiredItemAmount (Utilities|Struct|BreakBPS_Quest _array_element)))
        (Default|CompleteQuest _asbp_fp_hands (.RewardMoney (Utilities|Struct|BreakBPS_Quest _array_element)) (.RewardXP (Utilities|Struct|BreakBPS_Quest _array_element)) (.RewardUseful (Utilities|Struct|BreakBPS_Quest _array_element)))
        (goto _label Break)))
    (:Completed
      (if (not (== (LocalVariables|Getindex) -1))
        (Utilities|Array|RemoveIndex (Variables|Default|GetActiveQuests) (LocalVariables|Getindex))))))