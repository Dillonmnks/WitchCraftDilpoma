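; Interaction tracer component that finds the actor under the player camera's crosshair and relays interaction input to it.
; Every tick, a visibility line trace runs from the camera along its forward vector up to InteractionDistance.
; When the hit actor changes or is lost, toggle-focus messages notify the old and new actors, and FocusedActor is updated.
; The interact and left-mouse input actions send their respective interface messages to the valid focused actor.
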(event Input|EnhancedActionEvents|EnhancedInputActionIA_MyInteract
  (params (ActionValue :type Boolean) (ElapsedSeconds :type Float%20%28double-precision%29) (TriggeredSeconds :type Float%20%28double-precision%29) (InputAction :type Input%20Action%20Object%20Reference :default "/Game/Player/InputActions/IA_MyInteract.IA_MyInteract"))
  (:Started
    (bind _focusedactor (Variables|Default|GetFocusedActor)
      (:then
        (Class|BPIInteractable|InteractNEW(Message) _focusedactor))
      (:else))))

(event Input|EnhancedActionEvents|EnhancedInputActionIA_MyLMB
  (params (ActionValue :type Boolean) (ElapsedSeconds :type Float%20%28double-precision%29) (TriggeredSeconds :type Float%20%28double-precision%29) (InputAction :type Input%20Action%20Object%20Reference :default "/Game/Player/InputActions/IA_MyLMB.IA_MyLMB"))
  (bind _focusedactor (Variables|Default|GetFocusedActor)
    (:then
      (Class|BPIInteractable|LMBInteract(Message) _focusedactor))
    (:else)))

(event EventTick
  (params (DeltaSeconds :type Float%20%28single-precision%29))
  (CallFunction|Trace))

(fn Trace
  (bind _returnvalue (Game|GetPlayerCameraManager 0))
  (bind _returnvalue_2 (Transformation|GetActorLocation _returnvalue))
  (bind (_outhit _returnvalue_3) (Collision|LineTraceByChannel _returnvalue_2 (+ _returnvalue_2 (* (Math|Vector|GetForwardVector (Transformation|GetActorRotation _returnvalue)) (Variables|Default|GetInteractionDistance))) "TraceTypeQuery1" false 0 "None" true "(R=1.000000,G=0.000000,B=0.000000,A=1.000000)" "(R=0.000000,G=1.000000,B=0.000000,A=1.000000)" 3.0))
  (if _returnvalue_3
    (if (!= (Variables|Default|GetFocusedActor) (.HitActor (Collision|BreakHitResult _outhit)))
      (CallFunction|ToggleFocus)
      (Variables|Default|SetFocusedActor (.HitActor (Collision|BreakHitResult _outhit)))
      (CallFunction|ToggleFocus))
    (else
      (CallFunction|ToggleFocus)
      (Variables|Default|SetFocusedActor 0))))

(fn ToggleFocus
  (bind _focusedactor (Variables|Default|GetFocusedActor)
    (:then
      (Class|BPIInteractable|ToggleFocus(Message) _focusedactor))
    (:else
      (Variables|Default|SetFocusedActor 0))))