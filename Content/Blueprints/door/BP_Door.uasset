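; BP_Door is a door Blueprint that swings open once enough coins have been collected.
; A CollectCoins event increments a counter, and OpenDoorCheck compares it to CoinsNeeded, firing the open event only once through a DoOnce.
; Opening plays a timeline that lerps the Door component's relative yaw from closed to 120 degrees.
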(event Custom|opendoor
  (bind _open_anim (Timeline|dooranimation Play)
    (:Update
      (Transformation|SetRelativeRotation (Variables|Default|Getdoor) (Math|Rotator|MakeRotator 0.0 0.0 (Math|Float|Lerp 0.0 1.2e+02 _open_anim)) false false))))

(event Custom|CollectCoins
  (Math|Integer|IncrementInt (Variables|Default|GetCoinsCollected)))

(event Custom|OpenDoorCheck
  (if (>= (Variables|Default|GetCoinsCollected) (Variables|Default|GetCoinsNeeded))
    (Utilities|FlowControl|DoOnce false
      (:Completed
        (CallFunction|Opendoor)))))

(fn ConstructionScript)