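; BP_MailBox1 is an interactable mailbox actor that acts as a quest giver.
; Focus toggles custom depth rendering on its static mesh, and it exposes its Widget component as the interaction widget.
; Interaction is delegated to QuestGiverComponent through InterfaceInteract.
; An unconnected leftover in the event graph looks up quest data and opens a W_QuestGiver widget, but never runs.
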(event EventInterfaceToggleFocus
  (params (Focus :type Boolean))
  (Rendering|SetRenderCustomDepth (Variables|Default|GetStaticMesh) Focus))

(fn ConstructionScript)

(fn GetInteractionWidgetRef
  (return (Variables|Default|GetWidget)))

(fn InterfaceInteract
  (bind _objectiveid (Default|InterfaceInteract (Variables|Default|GetQuestGiverComponent)))
  (return _objectiveid))