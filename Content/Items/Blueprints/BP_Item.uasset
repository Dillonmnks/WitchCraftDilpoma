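; BP_Item is an interactable pickup for flower items such as Powa Flowa and Mantis Plantis.
; Construction maps ItemType to a DT_Items row, then applies that item's mesh.
; Focus toggles custom depth on the mesh, while interaction calls InteractOnServer to flip InteractToggle.
; Its OnRep hands the item to player 0's BP_MyCharacter via PickUpItem and sets AutoDestroyWhenFinished when no quantity remains.
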(event Custom|InteractOnServer
  (Variables|Default|SetInteractToggle (not (Variables|Default|GetInteractToggle))))

(event EventInterfaceInteract
  (CallFunction|InteractonServer))

(event EventInterfaceToggleFocus
  (params (Focus :type Boolean))
  (Rendering|SetRenderCustomDepth (Variables|Default|GetStaticMesh) Focus))

(fn ConstructionScript
  (bind _childactor (Variables|Default|GetChildActor))
  (bind _childactor_2 (Variables|/Script/Engine.ChildActorComponent|GetChildActor _childactor))
  (CallFunction|UpdateItem)
  (Components|StaticMesh|SetStaticMesh (Variables|Default|GetStaticMesh) (.Mesh (Utilities|Struct|BreakS_Item (Variables|Default|GetItem))))
  (if (== _childactor_2 "/Game/Player/Interaction/InteractionArea/BP_InteractionAreaCustomShape.BP_InteractionAreaCustomShape")
    (bind _asbp_interaction_area_custom_shape (Utilities|Casting|CastToBP_InteractionAreaCustomShape _childactor_2))
    (Variables|/Game/Player/Interaction/InteractionArea/BP_InteractionAreaCustomShape.BP_InteractionAreaCustomShape_C|SetCustomShape _asbp_interaction_area_custom_shape 0)))

(fn OnRepInteractToggle
  (bind _asbp_my_character (Utilities|Casting|CastToBP_MyCharacter (Game|GetPlayerCharacter 0)))
  (Default|PickUpItem _asbp_my_character self)
  (if (<= (Utilities|Struct|BreakS_Item (Variables|Default|GetItem)) 0)
    (Variables|Default|SetbAutoDestroyWhenFinished true)))

(fn UpdateItem
  (switch Utilities|FlowControl|Switch|SwitchonE_Items (Variables|Default|GetItemType)
    (:NewEnumerator0
      (bind _returnvalue (Utilities|GetDataTableRow "/Game/Inventory_System/DT_Items.DT_Items" "ASO")
        (:then
          (Variables|Default|SetItem _returnvalue))))
    (:NewEnumerator1
      (bind _returnvalue_2 (Utilities|GetDataTableRow "/Game/Inventory_System/DT_Items.DT_Items" "IMG")
        (:then
          (Variables|Default|SetItem _returnvalue_2))))
    (:NewEnumerator2
      (bind _returnvalue_3 (Utilities|GetDataTableRow "/Game/Inventory_System/DT_Items.DT_Items" "IFB")
        (:then
          (Variables|Default|SetItem _returnvalue_3))))
    (:NewEnumerator3
      (bind _returnvalue_4 (Utilities|GetDataTableRow "/Game/Inventory_System/DT_Items.DT_Items" "LDL")
        (:then
          (Variables|Default|SetItem _returnvalue_4))))
    (:NewEnumerator4
      (bind _returnvalue_5 (Utilities|GetDataTableRow "/Game/Inventory_System/DT_Items.DT_Items" "MTP")
        (:then
          (Variables|Default|SetItem _returnvalue_5))))
    (:NewEnumerator5
      (bind _returnvalue_6 (Utilities|GetDataTableRow "/Game/Inventory_System/DT_Items.DT_Items" "NMS")
        (:then
          (Variables|Default|SetItem _returnvalue_6))))
    (:NewEnumerator6
      (bind _returnvalue_7 (Utilities|GetDataTableRow "/Game/Inventory_System/DT_Items.DT_Items" "PWF")
        (:then
          (Variables|Default|SetItem _returnvalue_7))))
    (:NewEnumerator7
      (bind _returnvalue_8 (Utilities|GetDataTableRow "/Game/Inventory_System/DT_Items.DT_Items" "RFP")
        (:then
          (Variables|Default|SetItem _returnvalue_8))))
    (:NewEnumerator8
      (bind _returnvalue_9 (Utilities|GetDataTableRow "/Game/Inventory_System/DT_Items.DT_Items" "SKT")
        (:then
          (Variables|Default|SetItem _returnvalue_9))))
    (:NewEnumerator9
      (bind _returnvalue_10 (Utilities|GetDataTableRow "/Game/Inventory_System/DT_Items.DT_Items" "VIV")
        (:then
          (Variables|Default|SetItem _returnvalue_10))))))

(fn GetInteractionWidgetRef
  (return (Variables|Default|GetWidget)))