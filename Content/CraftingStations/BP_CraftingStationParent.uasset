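; Base crafting station actor that highlights on focus, exposes an interaction widget and holds a recipe production queue.
; Interaction flips InteractToggle through a server event, but its OnRep is empty and the crafting-window HUD code is unwired.
; AddToProduction tops up a matching recipe slot to its limit, then AddToQueue creates capped slots while space remains.
; Reversed subtraction zeroes the remainder after a match, so that overflow never reaches new slots.
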(event Custom|InteractOnServer
  (Variables|Default|SetInteractToggle (not (Variables|Default|GetInteractToggle))))

(event EventInterfaceToggleFocus
  (params (Focus :type Boolean))
  (Rendering|SetRenderCustomDepth (Variables|Default|GetStaticMesh) Focus))

(event EventInterfaceInteract
  (CallFunction|InteractonServer))

(fn ConstructionScript)

(fn ToggleEnabled)

(fn OnRepInteractToggle)

(fn AddtoProduction
  (params (AddRecipe :type S%20Recipe%20Structure) (Amount :type Integer))
  (Variables|Default|SetAdd%20Recipe AddRecipe)
  (Variables|Default|SetAmount Amount)
  (for (_array_element _array_index) (Variables|Default|GetProductionQueue)
    (if (> (Variables|Default|GetAmount) 0)
      (if (Utilities|Enum|Equal(Enum) (Utilities|Struct|BreakS_Recipe (.Recipe (Utilities|Struct|BreakS_Recipe_Production_Queue _array_element))) (Utilities|Struct|BreakS_Recipe AddRecipe))
        (LocalVariables|SetFreeSpace (Math|Integer|Max(Integer) (- (Variables|Default|GetProductionQueueLimit) (.QueuedAmount (Utilities|Struct|BreakS_Recipe_Production_Queue _array_element)))))
        (Utilities|Array|SetArrayElem (Variables|Default|GetProductionQueue) _array_index (Utilities|Struct|MakeS_Recipe_Production_Queue AddRecipe (+ (Math|Integer|Min(Integer) (LocalVariables|GetFreeSpace) (Variables|Default|GetAmount)) (.QueuedAmount (Utilities|Struct|BreakS_Recipe_Production_Queue _array_element)))))
        (Variables|Default|SetAmount (Math|Integer|Max(Integer) (- (Math|Integer|Min(Integer) (LocalVariables|GetFreeSpace) (Variables|Default|GetAmount)) (Variables|Default|GetAmount)))))))
  (CallFunction|AddtoQueue))

(fn AddtoQueue
  (while (and (< (Utilities|Array|Length (Variables|Default|GetProductionQueue)) (Variables|Default|GetProductionQueueLength)) (> (Variables|Default|GetAmount) 0))
    (Utilities|Array|Add (Variables|Default|GetProductionQueue) (Utilities|Struct|MakeS_Recipe_Production_Queue (Variables|Default|GetAdd%20Recipe) (Math|Integer|Min(Integer) (Variables|Default|GetAmount) (Variables|Default|GetProductionQueueLimit))))
    (Variables|Default|SetAmount (- (Variables|Default|GetAmount) (Math|Integer|Min(Integer) (Variables|Default|GetAmount) (Variables|Default|GetProductionQueueLimit))))))

(fn GetInteractionWidgetRef
  (return (Variables|Default|GetWidget)))