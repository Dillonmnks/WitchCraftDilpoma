(event EventBeginPlay
  (|CallParentFunction) ; This node is disabled and will not be called.\nDrag off pins to build functionality.
)

(event EventTick
  (params (DeltaSeconds :type Float%20%28single-precision%29)))

(fn MerchantIntroduction
  (bind _foundwidgets (Widget|GetAllWidgetsOfClass "/Game/Petru/SaveandLoad/WB_TimeDisplay.WB_TimeDisplay_C" true))
  (bind _output_get (LocalVariables|SetNewLocalVar_0 _foundwidgets))
  (CallFunction|SetDialogBranch (Utilities|Select :Index (+ (Math|Conversions|ToInteger(Boolean) (and (>= (.Hours (Math|Timespan|BreakTimespan (Variables|/Game/Petru/SaveandLoad/WB_TimeDisplay.WB_TimeDisplay_C|GetWidgetTime (Utilities|Array|Get(acopy) _output_get)))) 5) (< (.Hours (Math|Timespan|BreakTimespan (Variables|/Game/Petru/SaveandLoad/WB_TimeDisplay.WB_TimeDisplay_C|GetWidgetTime (Utilities|Array|Get(acopy) _output_get)))) 15))) (* (Math|Conversions|ToInteger(Boolean) (and (>= (.Hours (Math|Timespan|BreakTimespan (Variables|/Game/Petru/SaveandLoad/WB_TimeDisplay.WB_TimeDisplay_C|GetWidgetTime (Utilities|Array|Get(acopy) _output_get)))) 15) (< (.Hours (Math|Timespan|BreakTimespan (Variables|/Game/Petru/SaveandLoad/WB_TimeDisplay.WB_TimeDisplay_C|GetWidgetTime (Utilities|Array|Get(acopy) _output_get)))) 22))) 2)) :Option%200 "Night" :Option%201 "Morning" :Option%202 "Afternoon" :Option%203 "Default") "NewEnumerator0")
  (CallFunction|OpenConversation))

(fn Dialogue
  (|CallParentFunction)
  (switch name (Variables|Default|GetActiveDialogueBranch)
    (:Morning
      (bind _state (CallFunction|AddDialogue "Merchant" "GoodMorning" (Utilities|Array|MakeArray)))
      (switch Utilities|FlowControl|Switch|SwitchonEDialogueState _state
        (:NewEnumerator0
          (CallFunction|ClearDialogueProgress)
          (CallFunction|CloseConversation))))
    (:Afternoon
      (if (Variables|Default|GetHasGivenItem?)
        (bind _state_2 (CallFunction|AddDialogue "Merchant" "Thank you for the mushrooms" (Utilities|Array|MakeArray)))
        (switch Utilities|FlowControl|Switch|SwitchonEDialogueState _state_2
          (:NewEnumerator0
            (CallFunction|ClearDialogueProgress)
            (CallFunction|CloseConversation)))
        (else
          (bind (_state_3 _optionsindex) (CallFunction|AddDialogue "Merchant" "I am so hungry, i would like to eat mushrooms when i am done for today. Do you want to eat together ?" (Utilities|Array|MakeArray "Sure" "No")))
          (switch Utilities|FlowControl|Switch|SwitchonEDialogueState _state_3
            (:NewEnumerator0
              (switch int _optionsindex
                (:0
                  (bind _state_4 (CallFunction|AddDialogue "Merchant" "Great come speak to me when you have collected the mushrooms" (Utilities|Array|MakeArray)))
                  (switch Utilities|FlowControl|Switch|SwitchonEDialogueState _state_4
                    (:NewEnumerator0
                      (if true
                        (bind (_state_5 _optionsindex_2) (CallFunction|AddDialogue "Merchant" "I see you collected the mushrooms. pls give it to me" (Utilities|Array|MakeArray "Sure" "No")))
                        (switch Utilities|FlowControl|Switch|SwitchonEDialogueState _state_5
                          (:NewEnumerator0
                            (switch int _optionsindex_2
                              (:0
                                (bind _state_6 (CallFunction|AddDialogue "Merchant" "Ah Wonderful, beautiful Mushrooms" (Utilities|Array|MakeArray)))
                                (switch Utilities|FlowControl|Switch|SwitchonEDialogueState _state_6
                                  (:NewEnumerator0
                                    (CallFunction|ClearDialogueProgress)
                                    (CallFunction|CloseConversation))
                                  (:NewEnumerator1
                                    (Variables|Default|SetHasGivenItem? true))))
                              (:1
                                (bind _state_7 (CallFunction|AddDialogue "Merchant" "Oh ok. speak to me if you change your mind" (Utilities|Array|MakeArray)))
                                (switch Utilities|FlowControl|Switch|SwitchonEDialogueState _state_7
                                  (:NewEnumerator0
                                    (CallFunction|RemoveDialogueProgress 1)
                                    (CallFunction|CloseConversation)))))))
                        (else
                          (bind _state_8 (CallFunction|AddDialogue "Merchant" "Come speak to me when you have collected the mushrooms" (Utilities|Array|MakeArray)))
                          (switch Utilities|FlowControl|Switch|SwitchonEDialogueState _state_8
                            (:NewEnumerator0
                              (CallFunction|RemoveDialogueProgress 1)
                              (CallFunction|CloseConversation))))))))
                (:1
                  (bind _state_9 (CallFunction|AddDialogue "Merchant" "Speak to me if you change your mind" (Utilities|Array|MakeArray)))
                  (switch Utilities|FlowControl|Switch|SwitchonEDialogueState _state_9
                    (:NewEnumerator0
                      (CallFunction|ClearDialogueProgress)
                      (CallFunction|CloseConversation))))))))))
    (:Night
      (bind _state_10 (CallFunction|AddDialogue "Merchant" "I am trying to sleep" (Utilities|Array|MakeArray)))
      (switch Utilities|FlowControl|Switch|SwitchonEDialogueState _state_10
        (:NewEnumerator0
          (CallFunction|ClearDialogueProgress)
          (CallFunction|CloseConversation))))))

(fn OpenConversation
  (bind _foundwidgets (Widget|GetAllWidgetsOfClass "/Game/Petru/SaveandLoad/WB_TimeDisplay.WB_TimeDisplay_C" true))
  (bind _output_get (Variables|Default|SetTime%20Display _foundwidgets))
  (CallFunction|SetDialogBranch (Utilities|Select :Index (+ (Math|Conversions|ToInteger(Boolean) (and (>= (.Hours (Math|Timespan|BreakTimespan (Variables|/Game/Petru/SaveandLoad/WB_TimeDisplay.WB_TimeDisplay_C|GetWidgetTime (Utilities|Array|Get(acopy) _output_get)))) 5) (< (.Hours (Math|Timespan|BreakTimespan (Variables|/Game/Petru/SaveandLoad/WB_TimeDisplay.WB_TimeDisplay_C|GetWidgetTime (Utilities|Array|Get(acopy) _output_get)))) 15))) (* (Math|Conversions|ToInteger(Boolean) (and (>= (.Hours (Math|Timespan|BreakTimespan (Variables|/Game/Petru/SaveandLoad/WB_TimeDisplay.WB_TimeDisplay_C|GetWidgetTime (Utilities|Array|Get(acopy) _output_get)))) 15) (< (.Hours (Math|Timespan|BreakTimespan (Variables|/Game/Petru/SaveandLoad/WB_TimeDisplay.WB_TimeDisplay_C|GetWidgetTime (Utilities|Array|Get(acopy) _output_get)))) 22))) 2)) :Option%200 "Night" :Option%201 "Morning" :Option%202 "Afternoon" :Option%203 "Default") "NewEnumerator0")
  (|CallParentFunction))

(fn Interact
  (return ""))