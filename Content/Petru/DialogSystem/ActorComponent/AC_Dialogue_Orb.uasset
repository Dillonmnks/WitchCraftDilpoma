(event EventBeginPlay)

(event EventTick
  (params (DeltaSeconds :type Float%20%28single-precision%29)))

(fn Dialogue
  (|CallParentFunction)
  (switch name (Variables|Default|GetActiveDialogueBranch)
    (:Default
      (bind _state (CallFunction|AddDialogue "Orb" "Hello, nice to meet you. I will help throughout the game and explain everything to you " (Utilities|Array|MakeArray "Continue")))
      (switch Utilities|FlowControl|Switch|SwitchonEDialogueState _state
        (:NewEnumerator0
          (bind _state_2 (CallFunction|AddDialogue "Orb" "First, familiarize yourself with the controls. Use Wasd to move in all directions and use the mouse to look around." (Utilities|Array|MakeArray "Continue")))
          (switch Utilities|FlowControl|Switch|SwitchonEDialogueState _state_2
            (:NewEnumerator0
              (bind _state_3 (CallFunction|AddDialogue "Orb" "As you have already noticed, you can use the E key to interact with things, be it to talk to someone or to collect items in your inventory, which you open with tab" (Utilities|Array|MakeArray "Continue")))
              (switch Utilities|FlowControl|Switch|SwitchonEDialogueState _state_3
                (:NewEnumerator0
                  (bind _state_4 (CallFunction|AddDialogue "Orb" "I already have the first task for you. I am dusty and I want you to brew me a dust removal potion. please go to the box and collect the item" (Utilities|Array|MakeArray "Continue")))
                  (switch Utilities|FlowControl|Switch|SwitchonEDialogueState _state_4
                    (:NewEnumerator0
                      (CallFunction|ClearDialogueProgress)
                      (CallFunction|CloseConversation)
                      (Variables|Default|SetisFinished? true))))))))))
    (:GivenObject
      (bind _state_5 (CallFunction|AddDialogue "Orb" (Utilities|Select :Index (Math|Random|RandomIntegerinRange 0 1) :Option%200 "You are my twizzy my slime for real" :Option%201 "Give me that lean gluck gluck") (Utilities|Array|MakeArray "Continue")))
      (switch Utilities|FlowControl|Switch|SwitchonEDialogueState _state_5
        (:NewEnumerator0
          (CallFunction|ClearDialogueProgress)
          (CallFunction|CloseConversation))))))