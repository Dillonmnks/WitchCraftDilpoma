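; BP_TestCube is a test cube actor that requests an item save once it comes to rest after being hit.
; A hit on the Cube component starts a looping timer that repeatedly checks the actor's velocity.
; When the speed drops below a small threshold, it clears the timer and calls SaveItemsMessage on the game instance.
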(event OnComponentHit(Cube)
  (params (HitComponent :type Primitive%20Component%20Object%20Reference) (OtherActor :type Actor%20Object%20Reference) (OtherComp :type Primitive%20Component%20Object%20Reference) (NormalImpulse :type Vector :default "0, 0, 0") (Hit :type Hit%20Result%20Structure%20%28by%20ref%29))
  (bind _returnvalue (Utilities|Time|SetTimerbyEvent (delegate Custom|CheckVelocity) 0.1 true))
  (Variables|Default|SetCheck%20velocity%20timer _returnvalue))

(event Custom|CheckVelocity
  (if (< (Math|Vector|VectorLength (Transformation|GetVelocity)) 3.0)
    (Utilities|Time|ClearandInvalidateTimerbyHandle (Variables|Default|GetCheck%20velocity%20timer))
    (Class|BPISaveGame|SaveItems(Message) (Game|GetGameInstance) true)))

(event EventBeginPlay)

(event Collision|EventActorBeginOverlap
  (params (OtherActor :type Actor%20Object%20Reference)))

(event EventTick
  (params (DeltaSeconds :type Float%20%28single-precision%29)))

(fn ConstructionScript)