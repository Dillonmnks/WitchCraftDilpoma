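; Save game Blueprint that stores and restores the player's quest progress.
; SaveQuestDetails records each quest's current stage and objective progress in a map keyed by quest ID.
; LoadQuests re-adds active quests through the quest log component, restores their saved details, then overwrites its active and completed lists.
; SaveQuestLog copies completed quests but sets the active list to None, leaving the log's active quests unused.
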(fn SaveQuestDetails
  (params (Quest :type %20Object%20Reference))
  (Utilities|Map|Add 0 (Variables|Default|GetQuestID Quest) (Utilities|Struct|MakeFallbackStruct (Variables|Default|GetCurrentObjectiveProgress Quest) (Variables|Default|GetCurrentStage Quest))))

(fn LoadQuests
  (params (Quest%20Log%20Component :type %20Object%20Reference))
  (for _array_element (Variables|Default|GetCurrentActiveQuests)
    (bind _returnvalue (CallFunction|AddNewQuest Quest%20Log%20Component _array_element))
    (Variables|Default|SetCurrentStage _returnvalue (.CurrentStage (Utilities|Struct|BreakFallbackStruct (.Value (Utilities|Map|Find 0 _array_element)))))
    (Variables|Default|SetCurrentObjectiveProgress _returnvalue (.Progress (Utilities|Struct|BreakFallbackStruct (.Value (Utilities|Map|Find 0 _array_element))))))
  (Variables|Default|SetCurrentActiveQuests Quest%20Log%20Component (Variables|Default|GetCurrentActiveQuests))
  (Variables|Default|SetCompletedQuests Quest%20Log%20Component (Variables|Default|GetCompletedQuests)))

(fn SaveQuestLog
  (params (QuestLog :type %20Object%20Reference))
  (Variables|Default|SetCurrentActiveQuests 0)
  (Variables|Default|SetCompletedQuests (Variables|Default|GetCompletedQuests QuestLog)))