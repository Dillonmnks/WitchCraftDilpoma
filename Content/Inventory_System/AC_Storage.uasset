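; Inventory storage component that holds a fixed-size array of SItem stacks, with an empty ID marking a free slot.
; Initialize fills a WB_InventoryNEW wrap box with one WB_StorageItem per slot, and UpdateUI copies Content back into those widgets.
; PickUpItem tops up matching stacks before filling empty slots.
; OnDrop moves or merges stacks between storages by writing both Content arrays and refreshing both UIs, rejecting mismatched items.
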(event EventInitialize
  (params (UI_Widget :type Widget%20Object%20Reference))
  (bind _aswb_inventory_new (Utilities|Casting|CastToWB_InventoryNEW UI_Widget)
    (:then
      (bind _output_get (Variables|Default|SetWidget _aswb_inventory_new))
      (Widget|Panel|ClearChildren (Variables|/Game/Inventory_System/WB_InventoryNEW.WB_InventoryNEW_C|GetWrapBox _output_get))
      (Utilities|Array|Resize (Variables|Default|GetContent) (Variables|Default|GetSize))
      (for (_array_element _array_index) (Variables|Default|GetContent)
        (bind _returnvalue (UserInterface|CreateWidget "/Game/Inventory_System/WB_StorageItem.WB_StorageItem_C" 0 _array_element _array_index self))
        (Widget|Panel|AddChild (Variables|/Game/Inventory_System/WB_InventoryNEW.WB_InventoryNEW_C|GetWrapBox (Variables|Default|GetWidget)) _returnvalue))
      (UserInterface|Viewport|AddtoViewport (Variables|Default|GetWidget) 0))
    (:CastFailed
      (Development|PrintString "Failed to set UI Widget reference."))))

(event EventUpdateUI
  (for (_array_element _array_index) (Class|PanelWidget|GetAllChildren (Variables|/Game/Inventory_System/WB_InventoryNEW.WB_InventoryNEW_C|GetWrapBox (Variables|Default|GetWidget)))
    (bind _aswb_storage_item (Utilities|Casting|CastToWB_StorageItem _array_element)
      (:then
        (Variables|/Game/Inventory_System/WB_StorageItem.WB_StorageItem_C|SetItem _aswb_storage_item (Utilities|Array|Get(acopy) (Variables|Default|GetContent) _array_index)))
      (:CastFailed
        (Development|PrintString "Failed to cast to StorageItem.")))))

(fn FindStackableSlots
  (params (ID :type String))
  (for (_array_element _array_index) (Variables|Default|GetContent)
    (if (and (Utilities|Enum|Equal(Enum) (.ID (Utilities|Struct|BreakS_Item _array_element)) ID) (< (.Quantity (Utilities|Struct|BreakS_Item _array_element)) (.MaxStackAmount (Utilities|Struct|BreakS_Item _array_element))))
      (Utilities|Array|Add (LocalVariables|Getslots) _array_index)))
  (return (LocalVariables|Getslots)))

(fn FindEmptySlots
  (for (_array_element _array_index) (Variables|Default|GetContent)
    (if (Utilities|Enum|Equal(Enum) (Utilities|Struct|BreakS_Item _array_element) "")
      (Utilities|Array|Add (LocalVariables|Getslots) _array_index)))
  (return (LocalVariables|Getslots)))

(fn TransferItem
  (params (fromInventory :type AC%20Storage%20Object%20Reference%20%28by%20ref%29) (fromIndex :type Integer) (toIndex :type Integer) (Item :type S%20Item%20Structure%20%28by%20ref%29))
  (bind _content (Variables|Default|GetContent))
  (bind _output (Utilities|Array|Get(acopy) _content toIndex))
  (bind (_id _name _thumbnail _mesh _quantity _maxstackamount) (Utilities|Struct|BreakS_Item _output))
  (if (Utilities|Enum|Equal(Enum) _id "")
    (LocalVariables|SetfreeSpace (Utilities|Struct|BreakS_Item Item))
    (else
      (LocalVariables|SetfreeSpace (- _maxstackamount _quantity))))
  (LocalVariables|SetaddedAmount (Math|Integer|Min(Integer) (LocalVariables|GetfreeSpace) (.Quantity (Utilities|Struct|BreakS_Item Item))))
  (Modify|RemoveatIndex fromInventory fromIndex (LocalVariables|GetaddedAmount))
  (Modify|AddatIndex toIndex (LocalVariables|GetaddedAmount)))

(fn RemoveatIndex
  (params (Index :type Integer%20%28by%20ref%29) (Amount :type Integer%20%28by%20ref%29))
  (bind _content (Variables|Default|GetContent))
  (bind _output (Utilities|Array|Get(acopy) _content Index))
  (bind (_id _name _thumbnail _mesh _quantity _maxstackamount) (Utilities|Struct|BreakS_Item _output))
  (bind _returnvalue (- _quantity Amount))
  (if (<= _returnvalue 0)
    (Utilities|Struct|SetmembersinS_Item _output "" "None" 0 0)
    (else
      (Utilities|Struct|SetmembersinS_Item _output _id _name _thumbnail _mesh _returnvalue _maxstackamount))))

(fn AddatIndex
  (params (Index :type Integer%20%28by%20ref%29) (Amount :type Integer%20%28by%20ref%29))
  (bind _content (Variables|Default|GetContent))
  (bind _output (Utilities|Array|Get(acopy) _content Index))
  (bind (_id _name _thumbnail _mesh _quantity _maxstackamount) (Utilities|Struct|BreakS_Item _output))
  (Utilities|Struct|SetmembersinS_Item _output _id _name _thumbnail _mesh (+ Amount _quantity) _maxstackamount))

(fn PickUpItem
  (params (Item :type BP%20Item%20Object%20Reference%20%28by%20ref%29))
  (bind _quantity (Utilities|Struct|BreakS_Item (Variables|/Game/Items/Blueprints/BP_Item.BP_Item_C|GetItem Item)))
  (bind (_id _name _thumbnail _mesh _quantity_2 _maxstackamount) (Utilities|Struct|BreakS_Item (Variables|/Game/Items/Blueprints/BP_Item.BP_Item_C|GetItem Item)))
  (bind _returnvalue (Math|Integer|Min(Integer) _quantity_2 _maxstackamount))
  (bind _output_get (LocalVariables|SetsameSlots (Searching|FindStackableSlots (Utilities|Struct|BreakS_Item (Variables|/Game/Items/Blueprints/BP_Item.BP_Item_C|GetItem Item)))))
  (bind _array_element (Utilities|Array|ForEachLoopwithBreak _output_get :!label _label)
    (:LoopBody
      (if (== (Utilities|Struct|BreakS_Item (Variables|/Game/Items/Blueprints/BP_Item.BP_Item_C|GetItem Item)) 0)
        (goto _label Break)
        (else
          (bind _output_get_2 (LocalVariables|SetaddAmount (Math|Integer|Min(Integer) (- (.MaxStackAmount (Utilities|Struct|BreakS_Item (Utilities|Array|Get(acopy) (Variables|Default|GetContent) _array_element))) (.Quantity (Utilities|Struct|BreakS_Item (Utilities|Array|Get(acopy) (Variables|Default|GetContent) _array_element)))) _quantity)))
          (Modify|AddatIndex _array_element _output_get_2)
          (Utilities|Struct|SetmembersinS_Item (Variables|/Game/Items/Blueprints/BP_Item.BP_Item_C|GetItem Item) (Math|Integer|Max(Integer) (- _quantity (LocalVariables|GetaddAmount)))))))
    (:Completed
      (bind _output_get_3 (LocalVariables|SetemptySlots (Searching|FindEmptySlots)))
      (bind _array_element_2 (Utilities|Array|ForEachLoopwithBreak _output_get_3 :!label _label_2)
        (:LoopBody
          (if (== _quantity_2 0)
            (goto _label_2 Break)
            (else
              (Utilities|Struct|SetmembersinS_Item (Utilities|Array|Get(acopy) (Variables|Default|GetContent) _array_element_2) _id _name _thumbnail _mesh _returnvalue _maxstackamount)
              (Utilities|Struct|SetmembersinS_Item (Variables|/Game/Items/Blueprints/BP_Item.BP_Item_C|GetItem Item) (- _quantity_2 _returnvalue)))))
        (:Completed
          (CallFunction|UpdateUI))))))

(fn OnDrop
  (params (ToIndex :type Integer) (FromInventory :type AC%20Storage%20Object%20Reference%20%28by%20ref%29) (FromIndex :type Integer) (Item :type S%20Item%20Structure))
  (bind _content (Variables|Default|GetContent))
  (bind _content_2 (Variables|Default|GetContent))
  (bind (_id _quantity) (Utilities|Struct|BreakS_Item Item))
  (bind (_id_2 _name _thumbnail _mesh _quantity_2 _maxstackamount) (Utilities|Struct|BreakS_Item Item))
  (bind (_id_3 _name_2 _thumbnail_2 _mesh_2 _quantity_3 _maxstackamount_2) (Utilities|Struct|BreakS_Item Item))
  (bind _output (Utilities|Array|Get(acopy) _content_2 ToIndex))
  (bind _output_2 (Utilities|Array|Get(acopy) _content ToIndex))
  (bind (_id_4 _name_3 _thumbnail_3 _mesh_3 _quantity_4 _maxstackamount_3) (Utilities|Struct|BreakS_Item _output))
  (bind _id_5 (Utilities|Struct|BreakS_Item _output_2))
  (if (Utilities|Enum|Equal(Enum) _id_5 "")
    (Utilities|Array|SetArrayElem (Variables|Default|GetContent) ToIndex (Utilities|Struct|MakeS_Item _id_3 _name_2 _thumbnail_2 _mesh_2 _quantity_3 _maxstackamount_2))
    (Utilities|Array|SetArrayElem (Variables|AC_Storage_C|GetContent FromInventory) FromIndex (Utilities|Struct|MakeS_Item) :!label _label)
    (CallFunction|UpdateUI :!label _label_2)
    (CallFunction|UpdateUI FromInventory)
    (elif (Utilities|Enum|Equal(Enum) _id_5 _id)
      (bind _output_get (LocalVariables|SetTransferAmount (Math|Integer|Min(Integer) (- _maxstackamount_3 _quantity_4) _quantity)))
      (Utilities|Array|SetArrayElem (Variables|Default|GetContent) ToIndex (Utilities|Struct|MakeS_Item _id_4 _name_3 _thumbnail_3 _mesh_3 (+ _quantity_4 (LocalVariables|GetTransferAmount)) _maxstackamount_3))
      (if (<= (- _quantity _output_get) 0)
        (goto _label)
        (else
          (Utilities|Array|SetArrayElem (Variables|AC_Storage_C|GetContent FromInventory) FromIndex (Utilities|Struct|MakeS_Item _id_2 _name _thumbnail _mesh (- _quantity _output_get) _maxstackamount))
          (goto _label_2)))
      (else
        (Development|PrintString "Not matching items.")))))